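; Universe component that drives a SPICE-based space simulation, loading kernels and keeping the ephemeris time.
; Tick advances time with a sixth-power fast-forward curve, then takes the observer ID and offset from the focus object.
; Queries return body positions relative to that observer, divided by UniverseScale, plus orientations, radii and state vectors.
; Orbit helpers convert between conic elements and state vectors, apply delta-V impulses across reference frames and draw debug orbits.
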(event EventBeginPlay
  (CallFunction|Initialize))

(event EventTick
  (params (DeltaSeconds :type Float%20%28single-precision%29))
  (CallFunction|AdvanceET DeltaSeconds)
  (bind (_observer_spk_id _position_offset) (Default|GetPositionatEt (Variables|Universe|View|GetFocus%20Object) (Variables|State|Getet)))
  (Variables|Universe|View|SetObserver%20ID _observer_spk_id)
  (Variables|Universe|View|SetObserver%20Offset _position_offset))

(event EventSetFocus
  (params (New%20Focus :type Focusable%20Object%20BPI%20Interface))
  (Variables|Universe|View|SetFocus%20Object New%20Focus)
  (CallFunction|Initialize)
  (if false
    (bind _friendly_name (Default|GetName (Variables|Universe|View|GetFocus%20Object)))
    (Development|PrintString (Utilities|String|Append "Set Object Focus to: " _friendly_name) true true "(R=0.160182,G=0.900271,B=1.000000,A=1.000000)")))

(event EventSetFastForwardControl
  (params (Control%20Value :type Float%20%28double-precision%29))
  (Variables|Universe|View|SetTime%20Scale%20Control Control%20Value))

(fn Initialize
  (if (Variables|Universe|Internal|GetIs%20Initialized)
    (return)
    (else
      (Variables|Universe|Internal|SetIs%20Initialized true)
      (Utilities|FlowControl|Sequence
        (:then_0
          ;[1 1 1] Clear all kernel data and error states
          (Class|Spice|InitAll))
        (:then_1
          ;[1 1 1] Load core kernels one directory at a time
          (for _array_element (Variables|Universe|Config|GetCore%20Kernel%20Directories)
            (bind (_errormessage _kernelfilerelativepaths) (Class|Spice|EnumerateKernels _array_element)
              (:Success
                (bind _errormessage_2 (Class|Spice|FurnshList _kernelfilerelativepaths)
                  (:Success
                    (Development|PrintString (Utilities|String|Append "Loaded Kernel Directory: " _array_element)))
                  (:Error
                    (CallFunction|SetLastError _errormessage_2))))
              (:Error
                (CallFunction|SetLastError _errormessage)))))
        (:then_2
          ;[1 1 1] Load Additional Kernel Files Individually
          (for _array_element_2 (Variables|Universe|Config|GetAdditional%20Kernel%20Files)
            (bind _errormessage_3 (Class|Spice|Furnsh _array_element_2)
              (:Success
                (Development|PrintString (Utilities|String|Append "Loaded Kernel File: " _array_element_2)))
              (:Error
                (CallFunction|SetLastError _errormessage_3)))))
        (:then_3
          ;[1 1 1] Initialize the current Ephemeris Time
          (if (Variables|Universe|Config|GetInitialize%20ET%20To%20Current%20Time)
            (Variables|State|Setet (Class|Spice|EtNow))
            (else
              (bind (_errormessage_4 _et) (Class|Spice|Str2et (Variables|Universe|Config|GetET%20Initial%20Time))
                (:Success
                  (Variables|State|Setet _et)
                  (bind _utcstr (Class|Spice|Et2utc (Variables|State|Getet) "Calendar")
                    (:Success
                      (Development|PrintString (Utilities|String|Append "Time initialized to " _utcstr)))))
                (:Error
                  (CallFunction|SetLastError _errormessage_4))))))))))

(fn SetLastError
  (params (Last%20Error%20Message :type String))
  (bind _output_get (Variables|Universe|Internal|SetLast%20Error%20Message Last%20Error%20Message))
  (Development|PrintString _output_get true true "(R=1.000000,G=0.000000,B=0.000000,A=1.000000)" 4.0))

(fn AdvanceET
  (params (Delta%20Time :type Float%20%28double-precision%29))
  (Variables|State|Setet (+ (Variables|State|Getet) (Class|SpiceTypes|ToSEphemerisPeriod(Float) (* Delta%20Time (+ (* (Math|Float|Power (Variables|Universe|View|GetTime%20Scale%20Control) 6.0) (Variables|Universe|Config|GetMax%20Time%20Multiplier)) 1.0))))))

(fn ApplyImpulsetoOrbit
  (params (Orbit :type S%20Conic%20Elements%20Structure) (Orbit%20Reference%20Frame :type String) (Impulse :type Vector :default "0, 0, 0"))
  (LocalVariables|SetImpulse%20In%20Orbital%20Frame (Class|SpiceTypes|ToSVelocityVector(Vector) Impulse))
  (Utilities|FlowControl|Sequence
    (:then_0
      ;[1 1 1] If the orbit is in a different reference frame, we need to tranform the impule into that frame.
      (if (!= Orbit%20Reference%20Frame (Variables|Universe|View|GetReference%20Frame))
        (bind (_errormessage _rotate) (Class|Spice|Pxform (Variables|State|Getet) (Variables|Universe|View|GetReference%20Frame) Orbit%20Reference%20Frame)
          (:Success
            (LocalVariables|SetImpulse%20In%20Orbital%20Frame (|Mxv (LocalVariables|GetImpulse%20In%20Orbital%20Frame) _rotate)))
          (:Error
            (return "" false _errormessage)))))
    (:then_1
      ;[1 1 1] Add the Delta-V to the State Vector's velocity, and compute new orbital elements
      (bind (_errormessage_2 _state) (Class|Spice|Conics Orbit (Variables|State|Getet))
        (:Success
          (bind _elts (Class|Spice|Oscelt (Utilities|Struct|MakeSStateVector (.r (Utilities|Struct|BreakSStateVector _state)) (+ (.v (Utilities|Struct|BreakSStateVector _state)) (LocalVariables|GetImpulse%20In%20Orbital%20Frame))) (Variables|State|Getet) (.GravitationalParameter (Utilities|Struct|BreakSConicElements Orbit)))
            (:Success
              (return _elts true ""))))
        (:Error
          (return "" false _errormessage_2))))))

(fn Begin
  (CallFunction|Initialize)
  (return))

(fn DrawDebugOrbit
  (params (Orbit :type S%20Conic%20Elements%20Structure) (Orbit%20Reference%20Frame :type String) (Ref%20Body%20Ephemeris%20Id :type String) (Color :type Linear%20Color%20Structure))
  (Utilities|FlowControl|Sequence
    (:then_0
      (bind (_position _success _error_message) (CallFunction|GetEphemerisPosition Ref%20Body%20Ephemeris%20Id))
      (if _success
        (LocalVariables|SetLocal%20Transform (Math|Transform|MakeTransform _position "0, 0, 0" (Math|Conversions|ToVector(Float) (/ 1.0 (Class|SpiceTypes|ToFloat(SDistance) (Variables|Universe|View|GetUniverse%20Scale))))))
        (else
          (return false _error_message))))
    (:then_1
      (Class|SpiceOrbits|RenderDebugOrbit (Components|GetOwner) (LocalVariables|GetLocal%20Transform) (Variables|State|Getet) Orbit Orbit%20Reference%20Frame (Variables|Universe|View|GetReference%20Frame) (Math|Conversions|ToColor(LinearColor) Color) 0.0)
      (return true ""))))

(fn GetEphemerisPosition
  (params (Spk%20Id :type String))
  (bind (_errormessage _ptarg) (Class|Spice|Spkpos (Variables|State|Getet) Spk%20Id (Variables|Universe|View|GetObserver%20ID) (Variables|Universe|View|GetReference%20Frame) "None")
    (:Success
      (return (/ (Class|SpiceTypes|ToVector(SDistanceVector) (- _ptarg (Variables|Universe|View|GetObserver%20Offset))) (Class|SpiceTypes|ToFloat(SDistance) (Variables|Universe|View|GetUniverse%20Scale))) true ""))
    (:Error
      (return "0, 0, 0" false _errormessage))))

(fn GetEphemerisStateVector
  (params (Ephemeris%20Id :type String) (Parent%20Ephemeris%20Id :type String))
  (bind (_errormessage _state) (Class|Spice|Spkezr (Variables|State|Getet) Ephemeris%20Id Parent%20Ephemeris%20Id (Variables|Universe|View|GetReference%20Frame) "None")
    (:Success
      (return _state (Variables|Universe|View|GetReference%20Frame) true ""))
    (:Error
      (return "" "" false _errormessage))))

(fn GetEphemerisTime
  (return (Variables|State|Getet)))

(fn GetFastForwardControl
  (return (Variables|Universe|View|GetTime%20Scale%20Control)))

(fn GetFocus
  (return (Variables|Universe|View|GetFocus%20Object)))

(fn GetOrbitPosition
  (params (Orbit :type S%20Conic%20Elements%20Structure) (Reference%20Frame :type String) (Orbit%20Parent%20Ephemeris%20Id :type String))
  (Utilities|FlowControl|Sequence
    (:then_0
      ;[1 1 1] Get the position of the body this thing is orbiting
      (bind (_position _success _error_message) (CallFunction|GetEphemerisPosition Orbit%20Parent%20Ephemeris%20Id))
      (if _success
        (LocalVariables|SetOrbit%20Reference%20Location _position)
        (else
          (return "0, 0, 0" false _error_message))))
    (:then_1
      ;[1 1 1] Get the state vector/position from the orbit
      (bind (_state_vector _out_reference_frame _success_2 _error_message_2) (CallFunction|GetStateVectorfromOrbitalElements Orbit Reference%20Frame))
      (if _success_2
        (LocalVariables|SetState%20Vector%20Reference%20Frame _out_reference_frame)
        (bind _output_get (LocalVariables|SetState%20Vector _state_vector))
        (LocalVariables|Setr (.r (Utilities|Struct|BreakSStateVector _output_get)))
        (else
          (return "0, 0, 0" false _error_message_2))))
    (:then_2
      ;[1 1 1] If the orbit is in a different reference frame than the observer's, transform the position into the observer's.
      (if (!= (LocalVariables|GetState%20Vector%20Reference%20Frame) (Variables|Universe|View|GetReference%20Frame))
        (bind (_errormessage _rotate) (Class|Spice|Pxform (Variables|State|Getet) (LocalVariables|GetState%20Vector%20Reference%20Frame) (Variables|Universe|View|GetReference%20Frame))
          (:Success
            (LocalVariables|Setr (|Mxv (LocalVariables|Getr) _rotate)))
          (:Error
            (return "0, 0, 0" false _errormessage)))))
    (:then_3
      ;[1 1 1] Scale the position and add it to the parent location
      (return (+ (/ (Class|SpiceTypes|ToVector(SDistanceVector) (LocalVariables|Getr)) (Class|SpiceTypes|ToFloat(SDistance) (Variables|Universe|View|GetUniverse%20Scale))) (LocalVariables|GetOrbit%20Reference%20Location)) true ""))))

(fn GetOrbitalElementsfromStateVector
  (params (State%20Vector :type S%20State%20Vector%20Structure) (In%20Reference%20Frame :type String) (GM :type S%20Mass%20Constant%20Structure))
  (bind _elts (Class|Spice|Oscelt State%20Vector (Variables|State|Getet) GM)
    (:Success
      (return _elts In%20Reference%20Frame))))

(fn GetOrientation
  (params (Body%20Fixed%20Frame%20Id :type String))
  (bind (_errormessage _rotate) (Class|Spice|Pxform (Variables|State|Getet) Body%20Fixed%20Frame%20Id (Variables|Universe|View|GetReference%20Frame))
    (:Success
      (bind (_errormessage_2 _q) (Class|Spice|M2q _rotate)
        (:Success
          (return (Class|KismetMathLibrary|QuatRotator (Class|SpiceTypes|ToQuat(SQuaternion) _q)) true ""))
        (:Error
          (return "0, 0, 0" false _errormessage_2))))
    (:Error
      (return "0, 0, 0" false _errormessage))))

(fn GetRadaii
  (params (Id :type String))
  (bind (_value _errormessage) (|Bodvrd "All" Id "RADII")
    (:Success
      (return _value true ""))
    (:Error
      (return "" false _errormessage))))

(fn GetStateVectorfromOrbitalElements
  (params (Orbit :type S%20Conic%20Elements%20Structure) (In%20Reference%20Frame :type String))
  (bind (_errormessage _state) (Class|Spice|Conics Orbit (Variables|State|Getet))
    (:Success
      (return _state In%20Reference%20Frame true ""))
    (:Error
      (return "" "" false _errormessage))))

(fn ScaleDistanceVector
  (params (Distance :type S%20Distance%20Vector%20Structure))
  (return (/ (Class|SpiceTypes|ToVector(SDistanceVector) Distance) (Class|SpiceTypes|ToFloat(SDistance) (Variables|Universe|View|GetUniverse%20Scale)))))