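; Actor component that keeps its owning actor pointed toward the world origin, based on an ephemeris position.
; Each tick it queries Universe for the position of its EphemerisId and, on success, sets the owner's rotation to look from there to zero.
; The look-at starts from the ephemeris position rather than the actor's own location.
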(event EventBeginPlay
  (|CallParentFunction) ; This node is disabled and will not be called.\nDrag off pins to build functionality.
)

(event EventTick
  (params (DeltaSeconds :type Float%20%28single-precision%29))
  (|CallParentFunction DeltaSeconds)
  (bind (_position _success) (Default|GetEphemerisPosition (Variables|Default|GetUniverse) (Variables|Default|GetEphemeris%20Id)))
  (if _success
    (Transformation|SetActorRotation (Components|GetOwner) (Math|Rotator|FindLookatRotation _position (Math|Vector|MakeVector 0.0 0.0 0.0)))))