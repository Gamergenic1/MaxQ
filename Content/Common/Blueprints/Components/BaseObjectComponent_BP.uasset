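; Base component for celestial objects in a SPICE-driven universe, providing a name badge, optional debug orbit and focus support.
; Initialize runs once to find and begin the Universe, load additional kernels, fetch the orbited body's GM and create the badge widget.
; Tick calls empty position and orientation stubs, draws the orbit through the Universe and projects the owner's location to place or hide the badge.
; SPICE and drawing failures go to SetErrorState for on-screen printing.
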(event EventBeginPlay
  (SpaceToolkit|Initialize))

(event EventTick
  (params (DeltaSeconds :type Float%20%28single-precision%29))
  (Utilities|FlowControl|Sequence
    (:then_0
      (SpaceToolkit|UpdatePosition))
    (:then_1
      (SpaceToolkit|UpdateOrientation))
    (:then_2
      (SpaceToolkit|DrawDebugOrbit))
    (:then_3
      (SpaceToolkit|UpdateBadge))))

(fn SetErrorState
  (params (Last%20Error :type String))
  ;[1 1 1] The object caused an error of some sort.  This is a great place for a breakpoint.
  (bind _output_get (Variables|Default|SetLast%20Error Last%20Error))
  (Development|PrintString _output_get true true "(R=1.000000,G=0.000000,B=0.000000,A=1.000000)" 4.0))

(fn UpdatePosition)

(fn UpdateOrientation)

(fn Initialize
  (if (not (Variables|Default|GetInitialized))
    (Variables|Default|SetInitialized true)
    (Utilities|FlowControl|Sequence
      (:then_0
        ;[1 1 1] Find the universe, so we know what time it is etc
        (bind _universe (CallFunction|GetUniverse true))
        (bind _output_get (Variables|Default|SetUniverse _universe))
        (Default|Begin _output_get))
      (:then_1
        ;[1 1 1] Load any additional kernels the object requires
        (bind _errormessage (Class|Spice|FurnshList (Variables|Default|GetAdditional%20Kernels%20To%20Load))
          (:Error
            (SpaceToolkit|SetErrorState _errormessage))))
      (:then_2
        ;[1 1 1] Get the Gravitational Constant of the body being orbited
        (if (Variables|Default|GetShow%20Debug%20Orbit)
          (bind (_errormessage_2 _returnvalue) (Class|Spice|BodvrdMass (Variables|Default|GetOrbit%20Parent%20Mass%20Id) "GM")
            (:Success
              (Variables|Default|SetGM _returnvalue))
            (:Error
              (SpaceToolkit|SetErrorState _errormessage_2)))))
      (:then_3
        ;[1 1 1] Create a name badge widget for the object
        (if (Utilities|IsValidClass (Variables|Default|GetName%20Badget%20Asset))
          (bind _returnvalue_2 (UserInterface|CreateWidget (Variables|Default|GetName%20Badget%20Asset) (Game|GetPlayerController 0)))
          (bind _output_get_2 (Variables|Default|SetName%20Badge _returnvalue_2))
          (bind _asbadge_widget_bpi (Utilities|Casting|CastToBadgeWidget_BPI _output_get_2))
          (Default|SetName _asbadge_widget_bpi (Variables|Default|GetFriendly%20Name) (Variables|Default|GetBadge%20Color) (Variables|Default|GetOrbit%20Color))
          (UserInterface|Viewport|AddtoViewport (Variables|Default|GetName%20Badge) (Variables|Default|GetBadge%20Z%20Order))
          (Class|UserWidget|SetAlignmentinViewport (Variables|Default|GetName%20Badge) "(X=0.500000,Y=0.500000)"))))))

(fn DrawDebugOrbit
  (if (Variables|Default|GetShow%20Debug%20Orbit)
    (bind (_succeeded _error_message) (Default|DrawDebugOrbit (Variables|Default|GetUniverse) (Variables|Default|GetOrbit) (Variables|Default|GetOrbit%20Reference%20Frame) (Variables|Default|GetOrbit%20Parent%20Ephemeris%20Id) (Variables|Default|GetOrbit%20Color)))
    (if (not _succeeded)
      (SpaceToolkit|SetErrorState _error_message))))

(fn UpdateBadge
  (bind _returnvalue (Game|GetPlayerController 0))
  (bind _returnvalue_2 (Components|GetOwner))
  (bind _returnvalue_3 (Transformation|GetActorLocation _returnvalue_2))
  (bind (_screenposition _returnvalue_4) (Class|GameplayStatics|ProjectWorldtoScreen _returnvalue _returnvalue_3 false))
  (Utilities|IsValid (Variables|Default|GetName%20Badge)
    (:Is%20Valid
      (Utilities|FlowControl|Sequence
        (:then_0
          (if _returnvalue_4
            (Class|UserWidget|SetPositioninViewport (Variables|Default|GetName%20Badge) _screenposition true)))
        (:then_1
          (Widget|SetVisibility (Variables|Default|GetName%20Badge) (select _returnvalue_4 "Visible" "Hidden")))))))

(fn FocusonMe
  (SpaceToolkit|Initialize)
  (Default|SetFocus (Variables|Default|GetUniverse) self)
  (return))

(fn GetName
  (return (Variables|Default|GetFriendly%20Name)))

(fn GetPositionatEt
  (params (et :type S%20Ephemeris%20Time%20Structure))
  (return "" ""))

(fn GetRadii
  (return (Variables|Default|GetRadaii)))