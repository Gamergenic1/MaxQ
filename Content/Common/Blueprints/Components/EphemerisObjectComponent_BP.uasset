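; Actor component that drives its owner's position, rotation and scale from Universe ephemeris data for a celestial body.
; Position and orientation updates query by ephemeris ID and body-fixed frame, optionally setting an error state on failure.
; UpdateScale divides the body's scaled radii by the mesh's half-extents to size the actor.
; With ShowDebugOrbit on, Tick derives orbital elements from the state vector relative to the orbit parent before calling parent Tick.
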(event EventBeginPlay
  (|CallParentFunction) ; This node is disabled and will not be called.\nDrag off pins to build functionality.
)

(event EventTick
  (params (DeltaSeconds :type Float%20%28single-precision%29))
  (Utilities|FlowControl|Sequence
    (:then_0
      (if (Variables|Default|GetShow%20Debug%20Orbit)
        (bind (_state_vector _reference_frame _success) (Default|GetEphemerisStateVector (Variables|Default|GetUniverse) (Variables|Default|GetBody%20Ephemeris%20Id) (Variables|Default|GetOrbit%20Parent%20Ephemeris%20Id)))
        (if _success
          (bind (_orbit _out_reference_frame) (Default|GetOrbitalElementsfromStateVector (Variables|Default|GetUniverse) _state_vector _reference_frame (Variables|Default|GetGM)))
          (Variables|Default|SetOrbit _orbit)
          (Variables|Default|SetOrbit%20Reference%20Frame _out_reference_frame))))
    (:then_1
      (|CallParentFunction DeltaSeconds))))

(fn UpdatePosition
  (if (Variables|Default|GetSet%20Position)
    (bind (_position _success _error_message) (Default|GetEphemerisPosition (Variables|Default|GetUniverse) (Variables|Default|GetBody%20Ephemeris%20Id)))
    (if _success
      (Transformation|SetActorLocation (Components|GetOwner) _position false false)
      (|CallParentFunction)
      (return)
      (elif (Variables|Default|GetError%20On%20Position%20Error)
        (CallFunction|SetErrorState _error_message)))))

(fn UpdateOrientation
  (if (Variables|Default|GetSet%20Orientation)
    (bind (_orientation _success _error_message) (Default|GetOrientation (Variables|Default|GetUniverse) (Variables|Default|GetBody%20Fixed%20Frame)))
    (if _success
      (Transformation|SetActorRotation (Components|GetOwner) _orientation)
      (|CallParentFunction)
      (return)
      (elif (Variables|Default|GetError%20On%20Orientation%20Error)
        (CallFunction|SetErrorState _error_message)))))

(fn GetPositionatEt
  (params (et :type S%20Ephemeris%20Time%20Structure))
  (return (Variables|Default|GetBody%20Ephemeris%20Id) ""))

(fn UpdateScale
  (params (Mesh :type Static%20Mesh%20Component%20Object%20Reference))
  (bind (_min _max) (Components|StaticMesh|GetLocalBounds Mesh))
  (CallFunction|Initialize)
  (bind (_radaii _succeeded _error_message) (Default|GetRadaii (Variables|Default|GetUniverse) (Variables|Default|GetBody%20Mass%20Id)))
  (if _succeeded
    (bind _scaled_vector (Default|ScaleDistanceVector (Variables|Default|GetUniverse) _radaii))
    (bind _output_get (Variables|Default|SetRadaii _scaled_vector))
    (Transformation|SetActorScale3D (Components|GetOwner) (/ _output_get (/ (- _max _min) "2.000000,2.000000,2.000000")))
    (else
      (Variables|Default|SetLast%20Error _error_message))))