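; Orbiting object component that moves its owning actor along a conic orbit around a parent ephemeris body, using SPICE-style orbital math.
; BeginPlay enables debug orbit display and rebuilds the orbital elements with the GM gravitational parameter.
; Each tick sets the actor's location from the Universe's orbit position, setting an error state on failure.
; GetPositionAtEt evaluates the conics at a given ephemeris time, returning an offset relative to the parent body.
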(event EventBeginPlay
  (Variables|Default|SetShow%20Debug%20Orbit true)
  (|CallParentFunction)
  (Variables|Default|SetOrbit (Utilities|Struct|MakeSConicElements (.PerifocalDistance (Utilities|Struct|BreakSConicElements (Variables|Default|GetOrbit))) (.Eccentricity (Utilities|Struct|BreakSConicElements (Variables|Default|GetOrbit))) (.Inclination (Utilities|Struct|BreakSConicElements (Variables|Default|GetOrbit))) (.LongitudeOfAscendingNode (Utilities|Struct|BreakSConicElements (Variables|Default|GetOrbit))) (.ArgumentOfPeriapse (Utilities|Struct|BreakSConicElements (Variables|Default|GetOrbit))) (.MeanAnomalyAtEpoch (Utilities|Struct|BreakSConicElements (Variables|Default|GetOrbit))) (.Epoch (Utilities|Struct|BreakSConicElements (Variables|Default|GetOrbit))) (Variables|Default|GetGM))))

(event EventTick
  (params (DeltaSeconds :type Float%20%28single-precision%29))
  (Utilities|FlowControl|Sequence
    (:then_0
      (bind (_position _success _error_message) (Default|GetOrbitPosition (Variables|Default|GetUniverse) (Variables|Default|GetOrbit) (Variables|Default|GetOrbit%20Reference%20Frame) (Variables|Default|GetOrbit%20Parent%20Ephemeris%20Id)))
      (if _success
        (Transformation|SetActorLocation (Components|GetOwner) _position false false)
        (else
          (CallFunction|SetErrorState _error_message))))
    (:then_1
      (|CallParentFunction DeltaSeconds))))

(fn GetPositionatEt
  (params (et :type S%20Ephemeris%20Time%20Structure))
  (bind (_errormessage _state) (Class|Spice|Conics (Variables|Default|GetOrbit) et)
    (:Success
      (return (Variables|Default|GetOrbit%20Parent%20Ephemeris%20Id) (.r (Utilities|Struct|BreakSStateVector _state))))
    (:Error
      (CallFunction|SetErrorState _errormessage))))