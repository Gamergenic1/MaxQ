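; Base component for objects in a SPICE-driven universe, providing shared registration, focus and extents, with stubbed name and position-at-ET queries.
; On BeginPlay it initializes once, finding the single Universe_BPI component on the GameState, registering with it and loading additional SPICE kernels.
; Tick calls empty position and orientation update functions.
; Lookup and kernel-load failures are stored and printed on screen in red.
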(event EventBeginPlay
  (SpaceToolkit|Initialize))

(event EventTick
  (params (DeltaSeconds :type Float%20%28single-precision%29))
  (Utilities|FlowControl|Sequence
    (:then_0
      (SpaceToolkit|UpdatePosition))
    (:then_1
      (SpaceToolkit|UpdateOrientation))))

(fn SetErrorState
  (params (Last%20Error :type String))
  (bind _output_get (Variables|Default|SetLast%20Error Last%20Error))
  (Development|PrintString _output_get true true "(R=1.000000,G=0.000000,B=0.000000,A=1.000000)" 4.0))

(fn UpdatePosition)

(fn UpdateOrientation)

(fn Initialize
  (bind _returnvalue (Game|GetGameState))
  (bind _returnvalue_2 (Class|Actor|GetComponentsbyInterface _returnvalue "/Game/Common/Blueprints/Interfaces/Universe_BPI.Universe_BPI_C"))
  (if (not (Variables|Default|GetInitialized))
    (Variables|Default|SetInitialized true)
    (Utilities|FlowControl|Sequence
      (:then_0
        ;[1 1 1] Find the Universe's component
        (if (== (Utilities|Array|Length _returnvalue_2) 1)
          (bind _asuniverse_bpi (Utilities|Casting|CastToUniverse_BPI (Utilities|Array|Get(acopy) _returnvalue_2))
            (:then
              (bind _output_get (Variables|Default|SetUniverse _asuniverse_bpi))
              (Default|Begin _output_get self))
            (:CastFailed
              (SpaceToolkit|SetErrorState "Universe Was not castable to Universe_BPI")))
          (else
            (SpaceToolkit|SetErrorState "Object requires one Universe_BPI Interface"))))
      (:then_1
        ;[1 1 1] Load any additional kernels the object requires
        (bind _errormessage (Class|Spice|FurnshList (Variables|Default|GetAdditional%20Kernels%20To%20Load))
          (:Error
            (SpaceToolkit|SetErrorState _errormessage)))))))

(fn FocusonMe
  (SpaceToolkit|Initialize)
  (Default|SetFocus (Variables|Default|GetUniverse) self)
  (return))

(fn GetExtents
  (return (Variables|Default|GetRadaii)))

(fn GetName
  (return ""))

(fn GetPositionatEt
  (params (et :type S%20Ephemeris%20Time%20Structure))
  (return "" ""))