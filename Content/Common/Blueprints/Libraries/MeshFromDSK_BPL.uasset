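; Blueprint function library that builds a procedural mesh of a body's surface from SPICE DSK shape kernels, with Phobos as the example.
; TesselateSurfaceMesh samples a one-degree longitude/latitude grid through Latsrf and Srfnrm for points and normals, then converts them to Unreal vectors with grid UVs and two triangles per cell.
; CreatePhobosMesh loads kernels, requiring phobos512.bds, and feeds those arrays into a ProceduralMeshComponent section.
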(fn TesselateSurfaceMesh
  (params (Target :type String) (FixRef :type String) (Min%20Longitude :type Integer) (Max%20Longitude :type Integer) (Min%20Latutude :type Integer) (Max%20Latitude :type Integer))
  (bind _indices (LocalVariables|GetIndices))
  (bind _returnvalue (- Max%20Longitude Min%20Longitude))
  (bind _returnvalue_2 (- Max%20Longitude Min%20Longitude))
  (bind _returnvalue_3 (- Max%20Latitude Min%20Latutude))
  (bind _returnvalue_4 (+ _returnvalue 1))
  (bind _returnvalue_5 (* 0 _returnvalue_4))
  (Class|Spice|FurnshList (LocalVariables|GetKernels)
    (:Success
      (for _index (range Min%20Longitude Max%20Longitude)
        (LocalVariables|SetLongitude (Class|SpiceTypes|Degrees2Angle (Math|Conversions|ToFloat(Integer) _index)))
        (for _index_2 (range Min%20Latutude Max%20Latitude)
          (LocalVariables|SetLatitude (Class|SpiceTypes|Degrees2Angle (Math|Conversions|ToFloat(Integer) _index_2)))
          (Utilities|Array|Add (LocalVariables|GetSurface%20Coords) (Utilities|Struct|MakeSLonLat (LocalVariables|GetLongitude) (LocalVariables|GetLatitude)))))
      (bind (_errormessage _srfpts) (Class|Spice|Latsrf (Utilities|Struct|MakeSEphemerisTime 0.0) (LocalVariables|GetSurface%20Coords) 0 "DSK" Target FixRef)
        (:Success
          (bind _output_get (LocalVariables|Setsrfpts _srfpts))
          (bind (_errormessage_2 _normls) (Class|Spice|Srfnrm (Utilities|Struct|MakeSEphemerisTime 0.0) _output_get 0 "DSK" Target FixRef)
            (:Success
              (LocalVariables|Setnormls _normls)
              (LocalVariables|Setlatitude%20stride (+ (- Max%20Latitude Min%20Latutude) 1))
              (Utilities|Array|Resize (LocalVariables|GetVertices) _returnvalue_5)
              (Utilities|Array|Resize (LocalVariables|GetNormals) _returnvalue_5)
              (Utilities|Array|Resize (LocalVariables|GetUVs) 0)
              (for _index_3 (range 0 _returnvalue_2)
                (bind _output_get_2 (LocalVariables|Setlat _index_3))
                (LocalVariables|Setadd%20triangles (< _output_get_2 _returnvalue_2))
                (for _index_4 (range 0 _returnvalue_3)
                  (bind _output_get_3 (LocalVariables|Setlong _index_4))
                  (LocalVariables|Setadd%20triangles (and (< _output_get_3 _returnvalue_3) (LocalVariables|Getadd%20triangles)))
                  (Utilities|FlowControl|Sequence
                    (:then_0
                      ;[1 1 1] Compute base vertex index
                      (bind _output_get_4 (LocalVariables|Setbase%20vertex (+ (* (LocalVariables|Getlat) (LocalVariables|Getlatitude%20stride)) (LocalVariables|Getlong))))
                      (if (>= _output_get_4 64619)
                        (Development|PrintString 0)))
                    (:then_1
                      ;[1 1 1] Transform the vertex position from D.P. RHS to S.P. LHS
                      (Utilities|Array|SetArrayElem (LocalVariables|GetVertices) (LocalVariables|Getbase%20vertex) (Class|SpiceTypes|ToVector(SDistanceVector) (Utilities|Array|Get(acopy) (LocalVariables|Getsrfpts) (LocalVariables|Getbase%20vertex)))))
                    (:then_2
                      ;[1 1 1] Transform the vertex normal from D.P. RHS to S.P. LHS
                      (Utilities|Array|SetArrayElem (LocalVariables|GetNormals) (LocalVariables|Getbase%20vertex) (Class|SpiceTypes|ToVector(SDimensionless) (Utilities|Array|Get(acopy) (LocalVariables|Getnormls) (LocalVariables|Getbase%20vertex)))))
                    (:then_3
                      ;[1 1 1] Compute a simple long/lat projection for tex coords
                      (Utilities|Array|SetArrayElem (LocalVariables|GetUVs) (LocalVariables|Getbase%20vertex) (Math|Vector2D|MakeVector2D (Math|Conversions|ToFloat(Integer) (/ (LocalVariables|Getlong) (- Max%20Longitude Min%20Latutude))) (Math|Conversions|ToFloat(Integer) (/ (LocalVariables|Getlat) (- Max%20Latitude Min%20Longitude))))))
                    (:then_4
                      (if (LocalVariables|Getadd%20triangles)
                        ;[1 1 1] Add Indices for this cell to form two triangles
                        (Utilities|FlowControl|Sequence
                          (:then_0
                            (Utilities|Array|Add _indices (+ (LocalVariables|Getbase%20vertex) 0)))
                          (:then_1
                            (Utilities|Array|Add _indices (+ (+ (LocalVariables|Getbase%20vertex) (LocalVariables|Getlatitude%20stride)) 0)))
                          (:then_2
                            (Utilities|Array|Add _indices (+ (LocalVariables|Getbase%20vertex) 1)))
                          (:then_3
                            (Utilities|Array|Add _indices (+ (LocalVariables|Getbase%20vertex) 1)))
                          (:then_4
                            (Utilities|Array|Add _indices (+ (+ (LocalVariables|Getbase%20vertex) (LocalVariables|Getlatitude%20stride)) 0)))
                          (:then_5
                            (Utilities|Array|Add _indices (+ (+ (LocalVariables|Getbase%20vertex) (LocalVariables|Getlatitude%20stride)) 1)))))))))
              (return (LocalVariables|GetVertices) (LocalVariables|GetIndices) (LocalVariables|GetNormals) (LocalVariables|GetUVs)))
            (:Error
              (Development|PrintString 0 _errormessage_2 true true "(R=1.000000,G=0.000000,B=0.000000,A=1.000000)"))))
        (:Error
          (Development|PrintString 0 _errormessage true true "(R=1.000000,G=0.000000,B=0.000000,A=1.000000)"))))))

(fn CreatePhobosMesh
  (params (Procedural%20Mesh%20Component :type Procedural%20Mesh%20Component%20Object%20Reference))
  ;[0 0 0 1 12] This Example requires kernel file "phobos512.bds".
  ;
  ; You can download it here:
  ;
  ; https://naif.jpl.nasa.gov/pub/naif/generic_kernels/dsk/satellites/
  ;
  ; It should be placed in the directory:
  ; Content\Spice\Common\Kernels
  (Class|Spice|FurnshList (LocalVariables|GetKernels)
    (:Success
      (bind (_mesh_vertices _mesh_indices _mesh_normals _mesh_uvs) (CallFunction|TesselateSurfaceMesh "PHOBOS" "IAU_PHOBOS" 0 360 1 179))
      (Class|ProceduralMeshComponent|CreateMeshSectionLinearColor Procedural%20Mesh%20Component 0 _mesh_vertices _mesh_indices _mesh_normals _mesh_uvs 0 0 0 0 0 false))
    (:Error
      (Development|PrintString 0 "This example requires kernel file \"phobos512.bds\" - see commends in MeshFromDSK_BPL" true true "(R=1.000000,G=0.000000,B=0.000000,A=1.000000)"))))