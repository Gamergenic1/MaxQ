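; Blueprint function library for the Spacetool Kit that provides a lookup for the game's Universe.
; Get Universe searches the Game State for components implementing Universe_BPI and requires exactly one match.
; It casts that component to the interface and calls Begin on it before returning it, so the lookup has side effects.
; A missing, duplicate or uncastable component yields an optional printed error.
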(fn GetUniverse
  (params (Print%20Error%20if%20Unfounded :type Boolean))
  (bind _returnvalue (Game|GetGameState))
  (bind _returnvalue_2 (Class|Actor|GetComponentsbyInterface _returnvalue "/Game/Common/Blueprints/Interfaces/Universe_BPI.Universe_BPI_C"))
  (if (== (Utilities|Array|Length _returnvalue_2) 1)
    (bind _asuniverse_bpi (Utilities|Casting|CastToUniverse_BPI (Utilities|Array|Get(acopy) _returnvalue_2))
      (:then
        (Default|Begin _asuniverse_bpi)
        (return _asuniverse_bpi))
      (:CastFailed
        (if Print%20Error%20if%20Unfounded
          (Development|PrintString 0 "Universe Was not castable to Universe_BPI" true true "(R=1.000000,G=0.000000,B=0.000000,A=1.000000)"))))
    (elif Print%20Error%20if%20Unfounded
      (Development|PrintString 0 "One Universe_BPI Interface must exist" true true "(R=1.000000,G=0.000000,B=0.000000,A=1.000000)"))))