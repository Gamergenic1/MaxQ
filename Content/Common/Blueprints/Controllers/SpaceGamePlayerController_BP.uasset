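; Player controller for the space game that builds the universe HUD and switches possession between the map pawn and orbiting object pawns.
; Initialize creates the HUD once, linking it to the Universe, but re-gathers pawns on each call, appending to ObjectPawns without clearing it.
; Map Toggle swaps views, while FocusNext and FocusPrevious cycle object pawns with a wrapping index outside map view.
; AddChildWidget attaches widgets to the HUD's left panel, and Quit exits.
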(event EventBeginPlay
  (CallFunction|Initialize)
  (CallFunction|ShoworHideMapPawn (Variables|Default|GetIsMapShowing)))

(event EventTick
  (params (DeltaSeconds :type Float%20%28single-precision%29)))

(event EventAddChildWidget
  (params (Child :type User%20Widget%20Object%20Reference))
  (CallFunction|Initialize)
  (Utilities|IsValid (Variables|Default|GetSubHudAnchor)
    (:Is%20Valid
      (Widget|Panel|AddChild (Variables|Default|GetSubHudAnchor) Child))))

(event Input|ActionEvents|InputActionQuit
  (params (Key :type Key%20Structure :default "None"))
  (:Pressed
    (Game|QuitGame 0 "Quit" false)))

(event Input|ActionEvents|InputActionMapToggle
  (params (Key :type Key%20Structure :default "None"))
  (:Pressed
    (CallFunction|ShoworHideMapPawn (not (Variables|Default|GetIsMapShowing)))))

(event Input|ActionEvents|InputActionFocusNext
  (params (Key :type Key%20Structure :default "None"))
  (:Pressed
    (if (not (Variables|Default|GetIsMapShowing))
      (bind _pawn (CallFunction|GetNextObjectPawn 1))
      (Pawn|Possess _pawn))))

(event Input|ActionEvents|InputActionFocusPrevious
  (params (Key :type Key%20Structure :default "None"))
  (:Pressed
    (if (not (Variables|Default|GetIsMapShowing))
      (bind _pawn (CallFunction|GetNextObjectPawn -1))
      (Pawn|Possess _pawn))))

(fn ConstructionScript)

(fn Initialize
  (Utilities|FlowControl|Sequence
    (:then_0
      (if (not (Variables|Default|GetInitialized))
        (Variables|Default|SetInitialized true)
        (bind _universe (CallFunction|GetUniverse true))
        (Variables|Default|SetUniverse _universe)
        (bind _returnvalue (UserInterface|CreateWidget (Variables|Default|GetHudWidgetAsset) self))
        (bind _output_get (Variables|Default|SetHudWidget _returnvalue))
        (UserInterface|Viewport|AddtoViewport _output_get 0)
        (Widget|SetVisibility (Variables|Default|GetHudWidget) "Visible")
        (bind _asuniverse_hudwidget_bp (Utilities|Casting|CastToUniverseHUDWidget_BP (Variables|Default|GetHudWidget)))
        (Variables|/Game/Common/UI/UniverseHUDWidget_BP.UniverseHUDWidget_BP_C|SetUniverseState _asuniverse_hudwidget_bp (Variables|Default|GetUniverse))
        (Variables|Default|SetSubHudAnchor (Variables|/Game/Common/UI/UniverseHUDWidget_BP.UniverseHUDWidget_BP_C|GetLeftPanel _asuniverse_hudwidget_bp))))
    (:then_1
      (bind _returnvalue_2 (Actor|GetActorOfClass "/Game/Common/Blueprints/Pawns/MapViewPawn_BP.MapViewPawn_BP_C"))
      (Variables|Default|SetMap%20Pawn _returnvalue_2))
    (:then_2
      (bind _outactors (Actor|GetAllActorsOfClass "/Game/Common/Blueprints/Pawns/OrbitingPawn_BP.OrbitingPawn_BP_C"))
      (for _array_element _outactors
        (bind _aspawn (Utilities|Casting|CastToPawn _array_element))
        (Utilities|Array|Add (Variables|Default|GetObject%20Pawns) _aspawn)))))

(fn ShoworHideMapPawn
  (params (Show%20Map :type Boolean))
  (bind _output_get (Variables|Default|SetIsMapShowing Show%20Map))
  (if _output_get
    (Pawn|Possess (Variables|Default|GetMap%20Pawn))
    (else
      (bind _pawn (CallFunction|GetNextObjectPawn))
      (Pawn|Possess _pawn))))

(fn GetNextObjectPawn
  (params (Offset :type Integer))
  (bind _object_pawns (Variables|Default|GetObject%20Pawns))
  (bind _returnvalue (Utilities|Array|Length _object_pawns))
  (bind _output_get (Variables|Default|SetCurrent%20Pawn%20Index (Math|Integer|%(Integer) (+ Offset (Variables|Default|GetCurrent%20Pawn%20Index) _returnvalue) _returnvalue)))
  (return (Utilities|Array|Get(acopy) (Variables|Default|GetObject%20Pawns) _output_get)))