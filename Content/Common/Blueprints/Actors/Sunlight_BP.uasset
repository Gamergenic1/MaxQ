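; Sunlight actor that dims its light as the sun moves farther from the object of focus.
; Each tick it sets the light component's intensity from the distance to origin reported by its PointsAtOriginComponentBP.
; The falloff follows an inverse-square law relative to a reference distance, clamped so intensity never exceeds the maximum illumination.
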(event EventBeginPlay)

(event EventTick
  (params (DeltaSeconds :type Float%20%28single-precision%29))
  ;[1 1 1] Scale sunlight intensity, so it falls off the farther away the sun moves from the object of focus.
  (Rendering|Components|Light|SetIntensity (Variables|Default|GetLightComponent) (* (Variables|Default|GetMaxIllumination) (Math|Float|Clamp(Float) (/ (Math|Float|Square (Variables|Default|GetDistanceAtMaxIllumination)) (Math|Float|Max(Float) (Math|Float|Square (Variables|/Game/Common/Blueprints/Components/PointsAtOriginComponent_BP.PointsAtOriginComponent_BP_C|GetDistance%20From%20Origin (Variables|Default|GetPointsAtOriginComponent_BP))) 1.0))))))

(fn ConstructionScript)