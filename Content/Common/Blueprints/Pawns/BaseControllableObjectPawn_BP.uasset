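; Base pawn for a controllable object with an orbiting-object component, providing an orbit camera and its own sub-HUD.
; Pitch and yaw input accumulate into the camera boom's rotation with clamped pitch, while zoom scales arm length proportionally within limits, both applied each tick.
; One-time initialization adds the sub-HUD through the player controller's HUD-owner interface and binds it to the orbiting object and Universe.
; Local possession toggles that sub-HUD's visibility.
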(event EventBeginPlay
  (CallFunction|Initialize))

(event Collision|EventActorBeginOverlap
  (params (OtherActor :type Actor%20Object%20Reference)))

(event EventTick
  (params (DeltaSeconds :type Float%20%28single-precision%29))
  (Utilities|FlowControl|Sequence
    (:then_0
      (CallFunction|UpdateCameraZoom DeltaSeconds))
    (:then_1
      (CallFunction|UpdateCameraOrbit DeltaSeconds))))

(event EventPossessed
  (params (NewController :type Controller%20Object%20Reference))
  (if (Pawn|IsLocalPlayerController NewController)
    (Utilities|IsValid (Variables|Default|GetSub%20Hud)
      (:Is%20Valid
        (Widget|SetVisibility (Variables|Default|GetSub%20Hud) "Visible")))))

(event EventUnpossessed
  (params (OldController :type Controller%20Object%20Reference))
  (if (Pawn|IsLocalPlayerController OldController)
    (Utilities|IsValid (Variables|Default|GetSub%20Hud)
      (:Is%20Valid
        (Widget|SetVisibility (Variables|Default|GetSub%20Hud) "Collapsed")))))

(event Input|AxisEvents|InputAxisCameraPitch
  (params (AxisValue :type Float%20%28single-precision%29))
  (Variables|Default|SetTotal%20Camera%20Pitch (Math|Float|ClampAngle (+ (* AxisValue (Variables|Default|GetCamera%20Orbit%20Sensitivity) (Utilities|Time|GetWorldDeltaSeconds)) (Variables|Default|GetTotal%20Camera%20Pitch)) -8e+01 8e+01)))

(event Input|AxisEvents|InputAxisCameraYaw
  (params (AxisValue :type Float%20%28single-precision%29))
  (Variables|Default|SetTotal%20Camera%20Yaw (+ (* AxisValue (Variables|Default|GetCamera%20Orbit%20Sensitivity) (Utilities|Time|GetWorldDeltaSeconds)) (Variables|Default|GetTotal%20Camera%20Yaw))))

(fn ConstructionScript)

(fn UpdateCameraOrbit
  (params (Delta%20Seconds :type Float%20%28single-precision%29))
  (Transformation|SetRelativeRotation (Variables|Default|GetCameraBoom) (Math|Rotator|MakeRotator 0.0 (Variables|Default|GetTotal%20Camera%20Pitch) (Variables|Default|GetTotal%20Camera%20Yaw)) false false))

(fn UpdateCameraZoom
  (params (Delta%20Seconds :type Float%20%28single-precision%29))
  (Variables|/Script/Engine.SpringArmComponent|SetTargetArmLength (Variables|Default|GetCameraBoom) (Math|Float|Clamp(Float) (- (Variables|/Script/Engine.SpringArmComponent|GetTargetArmLength (Variables|Default|GetCameraBoom)) (* Delta%20Seconds (Input|AxisValues|GetCameraZoom) (Variables|/Script/Engine.SpringArmComponent|GetTargetArmLength (Variables|Default|GetCameraBoom)))) (Variables|Default|GetMin%20Zoom) (Variables|Default|GetMax%20Zoom))))

(fn Initialize
  (if (not (Variables|Default|GetInitialized))
    (Variables|Default|SetInitialized true)
    (Utilities|FlowControl|Sequence
      (:then_0
        (bind _universe (CallFunction|GetUniverse true))
        (Variables|Default|SetUniverse _universe))
      (:then_1
        (if (Utilities|IsValidClass (Variables|Default|GetSub%20Hud%20Asset))
          (bind _ashudowner_bpi (Utilities|Casting|CastToHUDOwner_BPI (Game|GetPlayerController 0)))
          (bind _returnvalue (UserInterface|CreateWidget (Variables|Default|GetSub%20Hud%20Asset)))
          (bind _output_get (Variables|Default|SetSub%20Hud _returnvalue))
          (Default|AddChildWidget _ashudowner_bpi _output_get)
          (Widget|SetVisibility _output_get "Collapsed")
          (bind _asobject_sub_hudt_bpi (Utilities|Casting|CastToObjectSubHud_BPI _output_get))
          (Default|Bind _asobject_sub_hudt_bpi (Variables|Default|GetOrbitingObjectComponent) (Variables|Default|GetUniverse)))))))