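; Pawn for the Hubble telescope that follows an orbit around Earth defined by orbital elements.
; On BeginPlay it starts the universe, then uses SPICE calls to fetch Earth's radius and GM and convert the epoch to ephemeris time.
; These values and the pawn's element variables build the conic elements for OrbitingObjectComponent, with periapsis as radius plus perigee altitude.
; When possessed by a local player controller, it tells that component to focus on it.
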(event EventBeginPlay
  (|CallParentFunction)
  (bind _universe (CallFunction|GetUniverse true))
  (Default|Begin _universe)
  (bind _value (|Bodvrd "All" "EARTH" "RADII")
    (:Success
      (bind _et (Class|Spice|Str2et (Variables|Default|GetEpoch))
        (:Success
          (bind _value_2 (|Bodvrd "All" "EARTH" "GM")
            (:Success
              (Variables|/Game/Common/Blueprints/Components/BaseObjectComponent_BP.BaseObjectComponent_BP_C|SetOrbit (Variables|Default|GetOrbitingObjectComponent) (Utilities|Struct|MakeSConicElements (+ (.x (Utilities|Struct|BreakSDistanceVector _value)) (Variables|Default|GetPerigee%20Altitude)) (Variables|Default|GetEccentricity) (Variables|Default|GetInclination) (Variables|Default|GetRight%20Ascension%20of%20Ascending%20Node) (Variables|Default|GetArgument%20of%20Perigee) (Variables|Default|GetMean%20Anomaly%20At%20Epoch) _et _value_2)))))))))

(event Collision|EventActorBeginOverlap
  (params (OtherActor :type Actor%20Object%20Reference))
  (|CallParentFunction OtherActor) ; This node is disabled and will not be called.\nDrag off pins to build functionality.
)

(event EventTick
  (params (DeltaSeconds :type Float%20%28single-precision%29))
  (|CallParentFunction DeltaSeconds))

(event EventPossessed
  (params (NewController :type Controller%20Object%20Reference))
  (|CallParentFunction NewController)
  (if (Pawn|IsLocalPlayerController NewController)
    (Default|FocusonMe (Variables|Default|GetOrbitingObjectComponent))))

(fn ConstructionScript
  (|CallParentFunction))