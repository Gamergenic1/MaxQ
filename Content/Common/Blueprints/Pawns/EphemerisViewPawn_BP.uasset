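; A view pawn that cycles its focus among the ephemeris objects in the level.
; On first BeginPlay or local possession it finds the game state's single Universe interface component and gathers the component of every EphemerisObject actor into a focus list.
; Next and previous body inputs step through that list with wraparound.
; Each newly focused object gets a FocusOnMe call, and the spring arm length scales to its largest extent.
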(event EventBeginPlay
  (CallFunction|Initialize))

(event Collision|EventActorBeginOverlap
  (params (OtherActor :type Actor%20Object%20Reference)))

(event EventTick
  (params (DeltaSeconds :type Float%20%28single-precision%29)))

(event EventPossessed
  (params (NewController :type Controller%20Object%20Reference))
  (if (Pawn|IsLocalPlayerController NewController)
    (CallFunction|Initialize)
    (bind _focusable (CallFunction|GetNextFocus))
    (Default|FocusonMe _focusable)
    (CallFunction|SetupCamera _focusable)))

(event Input|ActionEvents|InputActionBodyNext
  (params (Key :type Key%20Structure :default "None"))
  (:Pressed
    (bind _focusable (CallFunction|GetNextFocus 1))
    (Default|FocusonMe _focusable)
    (CallFunction|SetupCamera _focusable)))

(event Input|ActionEvents|InputActionBodyPrevious
  (params (Key :type Key%20Structure :default "None"))
  (:Pressed
    (bind _focusable (CallFunction|GetNextFocus -1))
    (Default|FocusonMe _focusable)
    (CallFunction|SetupCamera _focusable)))

(fn ConstructionScript)

(fn Initialize
  (bind _returnvalue (Game|GetGameState))
  (bind _returnvalue_2 (Class|Actor|GetComponentsbyInterface _returnvalue "/Game/Common/Blueprints/Interfaces/Universe_BPI.Universe_BPI_C"))
  (if (not (Variables|Default|GetInitialized))
    (Variables|Default|SetInitialized true)
    (Utilities|FlowControl|Sequence
      (:then_0
        ;[1 1 1] Find the Universe's component
        (if (== (Utilities|Array|Length _returnvalue_2) 1)
          (bind _asuniverse_bpi (Utilities|Casting|CastToUniverse_BPI (Utilities|Array|Get(acopy) _returnvalue_2))
            (:then
              (Variables|Default|SetUniverse _asuniverse_bpi))
            (:CastFailed
              (Development|PrintString "Universe Was not castable to Universe_BPI" true true "(R=1.000000,G=0.000000,B=0.000000,A=1.000000)")))
          (else
            (Development|PrintString "Object requires one Universe_BPI Interface" true true "(R=1.000000,G=0.000000,B=0.000000,A=1.000000)"))))
      (:then_1
        (bind _outactors (Actor|GetAllActorsOfClass "/Game/Common/Blueprints/Actors/EphemerisObject_BP.EphemerisObject_BP_C"))
        (for _array_element _outactors
          (Utilities|Array|Add (Variables|Default|GetFocus%20List) (Actor|GetComponentbyClass _array_element "/Game/Common/Blueprints/Components/EphemerisObjectComponent_BP.EphemerisObjectComponent_BP_C")))))))

(fn GetNextFocus
  (params (Offset :type Integer))
  (bind _focus_list (Variables|Default|GetFocus%20List))
  (bind _returnvalue (Utilities|Array|Length _focus_list))
  (bind _output_get (Variables|Default|SetFocus%20Current%20Index (Math|Integer|%(Integer) (+ (+ Offset (Variables|Default|GetFocus%20Current%20Index)) _returnvalue) _returnvalue)))
  (return (Utilities|Array|Get(acopy) (Variables|Default|GetFocus%20List) _output_get)))

(fn SetupCamera
  (params (New%20Focus%20Object :type Focusable%20Universe%20Object%20BPI%20Interface))
  (bind _radaii (Default|GetExtents New%20Focus%20Object))
  (Variables|/Script/Engine.SpringArmComponent|SetTargetArmLength (Variables|Default|GetSpringArm) (* (Math|Vector|GetMaxElement _radaii) 2.0)))