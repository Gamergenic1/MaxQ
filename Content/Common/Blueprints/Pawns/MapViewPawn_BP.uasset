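; Map view pawn that lets the player orbit and zoom a camera around ephemeris objects, cycling focus between them.
; On first initialization it gathers every ephemeris object component into a wrapping focus list and creates a HUD sub-widget bound to the universe, shown only while locally possessed.
; Each focus change scales spring arm length and minimum zoom to the object's extents.
; Tick applies distance-proportional zoom and pitch-clamped orbit from input.
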(event EventBeginPlay
  (CallFunction|Initialize))

(event Collision|EventActorBeginOverlap
  (params (OtherActor :type Actor%20Object%20Reference)))

(event EventTick
  (params (DeltaSeconds :type Float%20%28single-precision%29))
  (Utilities|FlowControl|Sequence
    (:then_0
      (CallFunction|UpdateCameraZoom DeltaSeconds))
    (:then_1
      (CallFunction|UpdateCameraOrbit DeltaSeconds))))

(event EventPossessed
  (params (NewController :type Controller%20Object%20Reference))
  (if (Pawn|IsLocalPlayerController NewController)
    (CallFunction|Initialize)
    (bind _focusable (CallFunction|GetNextFocus))
    (CallFunction|FocusonObject _focusable)
    (Utilities|IsValid (Variables|Default|GetSub%20Hud)
      (:Is%20Valid
        (Widget|SetVisibility (Variables|Default|GetSub%20Hud) "Visible")))))

(event EventUnpossessed
  (params (OldController :type Controller%20Object%20Reference))
  (if (Pawn|IsLocalPlayerController OldController)
    (Utilities|IsValid (Variables|Default|GetSub%20Hud)
      (:Is%20Valid
        (Widget|SetVisibility (Variables|Default|GetSub%20Hud) "Collapsed")))))

(event Input|ActionEvents|InputActionFocusNext
  (params (Key :type Key%20Structure :default "None"))
  (:Pressed
    (bind _focusable (CallFunction|GetNextFocus 1))
    (Default|FocusonMe _focusable)
    (CallFunction|SetupCamera _focusable)))

(event Input|ActionEvents|InputActionFocusPrevious
  (params (Key :type Key%20Structure :default "None"))
  (:Pressed
    (bind _focusable (CallFunction|GetNextFocus -1))
    (Default|FocusonMe _focusable)
    (CallFunction|SetupCamera _focusable)))

(fn ConstructionScript)

(fn Initialize
  (if (not (Variables|Default|GetInitialized))
    (Variables|Default|SetInitialized true)
    (Utilities|FlowControl|Sequence
      (:then_0
        (bind _universe (CallFunction|GetUniverse true))
        (Variables|Default|SetUniverse _universe))
      (:then_1
        (bind _outactors (Actor|GetAllActorsOfClass "/Game/Common/Blueprints/Actors/EphemerisObject_BP.EphemerisObject_BP_C"))
        (for _array_element _outactors
          (Utilities|Array|Add (Variables|Default|GetFocus%20List) (Actor|GetComponentbyClass _array_element "/Game/Common/Blueprints/Components/EphemerisObjectComponent_BP.EphemerisObjectComponent_BP_C"))))
      (:then_2
        (if (Utilities|IsValidClass (Variables|Default|GetSub%20Hud%20Asset))
          (bind _ashudowner_bpi (Utilities|Casting|CastToHUDOwner_BPI (Game|GetPlayerController 0)))
          (bind _returnvalue (UserInterface|CreateWidget (Variables|Default|GetSub%20Hud%20Asset)))
          (bind _output_get (Variables|Default|SetSub%20Hud _returnvalue))
          (Widget|SetVisibility _output_get "Collapsed")
          (Default|AddChildWidget _ashudowner_bpi _output_get)
          (bind _asmap_pawn_widget_bp (Utilities|Casting|CastToMapPawnWidget_BP _returnvalue))
          (Variables|/Game/Common/UI/MapPawnWidget_BP.MapPawnWidget_BP_C|SetUniverse _asmap_pawn_widget_bp (Variables|Default|GetUniverse)))))))

(fn GetNextFocus
  (params (Offset :type Integer))
  (bind _focus_list (Variables|Default|GetFocus%20List))
  (bind _returnvalue (Utilities|Array|Length _focus_list))
  (bind _output_get (Variables|Default|SetFocus%20Current%20Index (Math|Integer|%(Integer) (+ (+ Offset (Variables|Default|GetFocus%20Current%20Index)) _returnvalue) _returnvalue)))
  (return (Utilities|Array|Get(acopy) (Variables|Default|GetFocus%20List) _output_get)))

(fn SetupCamera
  (params (New%20Focus%20Object :type Focusable%20Universe%20Object%20BPI%20Interface))
  (bind _radaii (Default|GetExtents New%20Focus%20Object))
  (bind _output_get (Variables|Default|SetMinCameraDistance (* (Math|Vector|GetMaxElement _radaii) 3.0)))
  (Variables|/Script/Engine.SpringArmComponent|SetTargetArmLength (Variables|Default|GetSpringArm) (* _output_get 3.0)))

(fn FocusonObject
  (params (Focusable :type Focusable%20Universe%20Object%20BPI%20Interface))
  (Utilities|FlowControl|Sequence
    (:then_0
      (Default|FocusonMe Focusable))
    (:then_1
      (CallFunction|SetupCamera Focusable))))

(fn UpdateCameraZoom
  (params (Delta%20Seconds :type Float%20%28single-precision%29))
  (Variables|/Script/Engine.SpringArmComponent|SetTargetArmLength (Variables|Default|GetSpringArm) (Math|Float|Clamp(Float) (- (Variables|/Script/Engine.SpringArmComponent|GetTargetArmLength (Variables|Default|GetSpringArm)) (* (* Delta%20Seconds (Input|AxisValues|GetCameraZoom)) (Variables|/Script/Engine.SpringArmComponent|GetTargetArmLength (Variables|Default|GetSpringArm)))) (Variables|Default|GetMinCameraDistance) (Variables|Default|GetMaxCameraDistance))))

(fn UpdateCameraOrbit
  (params (Delta%20Seconds :type Float%20%28single-precision%29))
  (bind _springarm (Variables|Default|GetSpringArm))
  (bind _camera_orbit_sensitivity (Variables|Default|GetCamera%20Orbit%20Sensitivity))
  (bind _returnvalue (Transformation|GetWorldRotation _springarm))
  (bind (_roll _pitch _yaw) (Math|Rotator|BreakRotator _returnvalue))
  (Transformation|SetWorldRotation (Variables|Default|GetSpringArm) (Math|Rotator|MakeRotator 0.0 (Math|Float|ClampAngle (+ _pitch (* (* (Input|AxisValues|GetCameraPitch) _camera_orbit_sensitivity) Delta%20Seconds)) -8e+01 8e+01) (+ _yaw (* Delta%20Seconds (* _camera_orbit_sensitivity (Input|AxisValues|GetCameraYaw))))) false false))