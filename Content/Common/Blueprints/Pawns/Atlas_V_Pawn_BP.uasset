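; Player-flyable Atlas V rocket pawn that maneuvers as an orbiting object, with upper-stage exhaust effects.
; Each tick, throttle drives the Niagara plume and engine light and applies an impulse along the actor's up axis through OrbitingObjectComponent.
; Pitch, roll and yaw inputs rotate it in its local frame via quaternion multiplication, scaled by a fixed angular rate.
; Possession by a local player controller focuses the orbiting component on this pawn.
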(event EventBeginPlay
  (|CallParentFunction)
  (bind _returnvalue (Niagara|SpawnSystemAttached "/Game/Common/Effects/Atlas_5_401_UpperStageExhaust_Small_NS.Atlas_5_401_UpperStageExhaust_Small_NS" (Variables|Default|GetSkeletalMesh) "TC" "0, 0, 0" "0, 0, 0" "KeepRelativeOffset" false))
  (Variables|Default|SetThrust%20VFX _returnvalue))

(event Collision|EventActorBeginOverlap
  (params (OtherActor :type Actor%20Object%20Reference))
  (|CallParentFunction OtherActor) ; This node is disabled and will not be called.\nDrag off pins to build functionality.
)

(event EventTick
  (params (DeltaSeconds :type Float%20%28single-precision%29))
  (Utilities|FlowControl|Sequence
    (:then_0
      (CallFunction|ApplyThrottle DeltaSeconds))
    (:then_1
      (bind _out_rotation (CallFunction|ApplyRotation (Transformation|GetActorRotation) (Input|AxisValues|GetPitch) (Input|AxisValues|GetRoll) (Input|AxisValues|GetYaw) 1.8e+02 DeltaSeconds))
      (Transformation|SetActorRotation _out_rotation))
    (:then_2
      (|CallParentFunction DeltaSeconds))))

(event EventPossessed
  (params (NewController :type Controller%20Object%20Reference))
  (|CallParentFunction NewController)
  (if (Pawn|IsLocalPlayerController NewController)
    (Default|FocusonMe (Variables|Default|GetOrbitingObjectComponent))))

(fn ConstructionScript
  (|CallParentFunction))

(fn ApplyThrottle
  (params (Delta%20Seconds :type Float%20%28single-precision%29))
  (bind _returnvalue (Input|AxisValues|GetThrottle))
  (Rendering|Components|Light|SetIntensity (Variables|Default|GetThrust%20Illumination) (* _returnvalue 0.2))
  (Effects|Components|ParticleSystem|SetFloatParameter (Variables|Default|GetThrust%20VFX) "Throttle" _returnvalue)
  (if (> _returnvalue 0.0)
    (Default|ApplyImpulse (Variables|Default|GetOrbitingObjectComponent) (* (* Delta%20Seconds (Input|AxisValues|GetThrottle) (Variables|Default|GetMax%20Acceleration)) (Transformation|GetActorUpVector)))))

(fn ApplyRotation
  (params (In%20Rotation :type Rotator) (Pitch :type Float%20%28single-precision%29) (Roll :type Float%20%28single-precision%29) (Yaw :type Float%20%28single-precision%29) (Angular%20Rate :type Float%20%28single-precision%29) (Delta%20Seconds :type Float%20%28single-precision%29))
  (bind _returnvalue (* Angular%20Rate Delta%20Seconds))
  (return (Class|KismetMathLibrary|QuatRotator (* (Math|Conversions|ToQuaternion(Rotator) In%20Rotation) (Math|Conversions|ToQuaternion(Rotator) (Math|Rotator|MakeRotator (* Roll _returnvalue) (* Pitch _returnvalue) (* Yaw _returnvalue)))))))