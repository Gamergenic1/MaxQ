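; Demo actor that runs a catalog of the most commonly used SPICE (CSPICE) toolkit operations when play begins.
; BeginPlay uses nested sequences to step through seven printed categories, from kernel data access and derived geometry to event finding, coordinate conversions, vector math and constants.
; Each category calls one example function per topic, with InitAll run at the start and after nearly every example.
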(event EventBeginPlay
  (Class|Spice|InitAll)
  (Utilities|FlowControl|Sequence
    (:then_0
      (Development|PrintString "Accessing SPICE Kernel Data" true true "(R=1.000000,G=1.000000,B=0.000000,A=1.000000)")
      ;[1 1 1] Accessing SPICE Kernel Data
      (Utilities|FlowControl|Sequence
        (:then_0
          (CallFunction|LoadingandUnloadingSPICEKernels)
          (Class|Spice|InitAll))
        (:then_1
          (CallFunction|ConvertingBetweenUTCandEphemerisTime(LSK))
          (Class|Spice|InitAll))
        (:then_2
          (CallFunction|ConvertingBetweenEphemerisTimeandSpacecraftClock(SCLK))
          (Class|Spice|InitAll))
        (:then_3
          (CallFunction|RetrievingConstantsandOrientationforNaturalBodies(PCK))
          (Class|Spice|InitAll))
        (:then_4
          (CallFunction|ComputingTransformationsBetweenReferenceFrames(FK))
          (Class|Spice|InitAll))
        (:then_5
          (CallFunction|ComputingPositionsOfSpacecraftandNaturalBodies(SPK))
          (Class|Spice|InitAll))
        (:then_6
          (CallFunction|ComputingOrientationsOfSpacecraftandInstruments(CK))
          (Class|Spice|InitAll))
        (:then_7
          (CallFunction|RetrievingInstrumentParameters(IK))
          (Class|Spice|InitAll))
        (:then_8
          (CallFunction|ComputingSurfaceCoordinatesUsingDigitalShape(DSK))
          (Class|Spice|InitAll))
        (:then_9
          (CallFunction|MappingBetweenObjectNamesandNAIFIDs)
          (Class|Spice|InitAll))
        (:then_10
          (CallFunction|MappingBetweenSurfaceNamesandNAIFIDs)
          (Class|Spice|InitAll))))
    (:then_1
      (Development|PrintString "Computing Derived Geometry" true true "(R=1.000000,G=1.000000,B=0.000000,A=1.000000)")
      ;[1 1 1] Computing Derived Geometry
      (Utilities|FlowControl|Sequence
        (:then_0
          (CallFunction|ComputingPlanetocentric,Planetodetic,andPlanetographicCoordinates)
          (Class|Spice|InitAll))
        (:then_1
          (CallFunction|ComputingSurfaceInterceptPoint)
          (Class|Spice|InitAll))
        (:then_2
          (CallFunction|ComputingSub-observerandSub-solarPoints)
          (Class|Spice|InitAll))
        (:then_3
          (CallFunction|ComputingIlluminationAngles)
          (Class|Spice|InitAll))
        (:then_4
          (CallFunction|ComputingLimbandTerminator)
          (Class|Spice|InitAll))
        (:then_5
          (CallFunction|ComputingandPropagatingOrbitalElements)
          (Class|Spice|InitAll))))
    (:then_2
      (Development|PrintString "Checking geometric conditions" true true "(R=1.000000,G=1.000000,B=0.000000,A=1.000000)")
      ;[1 1 1] Checking geometric conditions
      (Utilities|FlowControl|Sequence
        (:then_0
          (CallFunction|CheckingforinField-Of-View(FOV)Conditions)
          (Class|Spice|InitAll))
        (:then_1
          (CallFunction|CheckingforOccultationConditions)
          (Class|Spice|InitAll))))
    (:then_3
      (Development|PrintString "Finding times of geometric events" true true "(R=1.000000,G=1.000000,B=0.000000,A=1.000000)")
      ;[1 1 1] Finding times of geometric events
      (Utilities|FlowControl|Sequence
        (:then_0
          (CallFunction|FindingTimesOfEventsSatisfyingNumericalConstraints)
          (Class|Spice|InitAll))
        (:then_1
          (CallFunction|FindingTimesOfEventsSatisfyingFOVConstraints)
          (Class|Spice|InitAll))
        (:then_2
          (CallFunction|FindingTimesOfOccultations)
          (Class|Spice|InitAll))))
    (:then_4
      (Development|PrintString "Coordinate Conversions" true true "(R=1.000000,G=1.000000,B=0.000000,A=1.000000)")
      ;[1 1 1] Coordinate Conversions
      (Utilities|FlowControl|Sequence
        (:then_0
          (CallFunction|ConvertingfromandtoRectangularCoordinates)
          (Class|Spice|InitAll))
        (:then_1
          (CallFunction|ConvertingfromandtoSphericalCoordinates)
          (Class|Spice|InitAll))
        (:then_2
          (CallFunction|ConvertingfromandtoCylindricalCoordinates)
          (Class|Spice|InitAll))
        (:then_3
          (CallFunction|ConvertingfromandtoLatitudinalCoordinates)
          (Class|Spice|InitAll))
        (:then_4
          (CallFunction|ConvertingfromandtoR,RA,DEC)
          (Class|Spice|InitAll))
        (:then_5
          (CallFunction|ConvertingfromandtoGeodeticCoordinates)
          (Class|Spice|InitAll))
        (:then_6
          (CallFunction|TransformingStatesfromOneCoordinateSystemtoAnother)
          (Class|Spice|InitAll))))
    (:then_5
      (Development|PrintString "Operations with 3D vectors and matrices" true true "(R=1.000000,G=1.000000,B=0.000000,A=1.000000)")
      ;[1 1 1] Operations with 3D vectors and matrices
      (Utilities|FlowControl|Sequence
        (:then_0
          (CallFunction|PerformingSimpleOperationson3DVectors)
          (Class|Spice|InitAll))
        (:then_1
          (CallFunction|PerformingSimpleOperationson3x3Matrices)
          (Class|Spice|InitAll))
        (:then_2
          (CallFunction|Projecting,CombiningandRotating3DVectors)
          (Class|Spice|InitAll))
        (:then_3
          (CallFunction|CreatingandConvertingTransformationMatrices)
          (Class|Spice|InitAll))))
    (:then_6
      (Development|PrintString "Miscellaneous CSPICE APIs" true true "(R=1.000000,G=1.000000,B=0.000000,A=1.000000)")
      ;[1 1 1] Miscellaneous CSPICE APIs
      (CallFunction|AccessingPhysicalandMathematicalConstants))))

(fn ConstructionScript)