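; Actor that, on BeginPlay, prints current range and RA/Dec for small bodies from a data table, sorted by range.
; It uses SPICE calls to load kernels and fetch the Sun's GM, then RowToOrbitalElements converts each row's units and epoch into conic elements.
; Conics propagates them to now; results are offset by the Earth-to-SSB vector, rotated from ECLIPJ2000 to J2000, then ordered through a Shell-sort index array.
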(event EventBeginPlay
  (bind _errormessage (Class|Spice|FurnshList (Variables|Default|GetRequired%20Kernels))
    (:Success
      (bind (_value _errormessage_2) (|Bodvrd "All" "SUN" "GM")
        (:Success
          (Variables|Default|SetGM _value)
          ;[1 1 1] Iterate through all records and compute state vectors
          (bind _outrownames (DataTable|GetDataTableRowNames (Variables|Default|GetSmallBodiesData)))
          (for _array_element _outrownames
            (bind _returnvalue (Utilities|GetDataTableRow (Variables|Default|GetSmallBodiesData) _array_element)
              (:then
                (bind _orbitalelements (CallFunction|RowtoOrbitalElements _returnvalue (Variables|Default|GetGM)))
                (bind _state (Class|Spice|Conics _orbitalelements (Class|Spice|EtNow))
                  (:Success
                    (bind _ptarg (Class|Spice|Spkpos (Class|Spice|EtNow) "SSB" "EARTH" "ECLIPJ2000" "None")
                      (:Success
                        (bind _rotate (Class|Spice|Pxform (Class|Spice|EtNow) "ECLIPJ2000" "J2000")
                          (:Success
                            (Utilities|Array|Add (Variables|Default|GetState%20Vectors) (Utilities|Struct|MakeStateVector_STRUCT (.full_name (Utilities|Struct|BreakSmallBodyRecord_STRUCT _returnvalue)) (.range (Class|Spice|Recrad (Class|Spice|MxvDistance _rotate (- (.r (Utilities|Struct|BreakSStateVector _state)) _ptarg)))) (.ra (Class|Spice|Recrad (Class|Spice|MxvDistance _rotate (- (.r (Utilities|Struct|BreakSStateVector _state)) _ptarg)))) (.dec (Class|Spice|Recrad (Class|Spice|MxvDistance _rotate (- (.r (Utilities|Struct|BreakSStateVector _state)) _ptarg))))))
                            (Utilities|Array|Add (Variables|Default|GetSortableRanges) (Class|SpiceTypes|ToFloat(SDistance) (.range (Class|Spice|Recrad (Class|Spice|MxvDistance _rotate (- (.r (Utilities|Struct|BreakSStateVector _state)) _ptarg)))))))))))))))
          (bind _order (Class|Spice|ShelldbyIndex (Variables|Default|GetSortableRanges)))
          (for (_ _array_index) (Variables|Default|GetState%20Vectors)
            (Development|PrintText (Utilities|Text|FormatText "{name} : Range {r} km; {radec}" (.Name (Utilities|Struct|BreakStateVector_STRUCT (Utilities|Array|Get(acopy) (Variables|Default|GetState%20Vectors) (Utilities|Array|Get(acopy) _order _array_index)))) (Class|SpiceTypes|ToString(SDistance) (.Range (Utilities|Struct|BreakStateVector_STRUCT (Utilities|Array|Get(acopy) (Variables|Default|GetState%20Vectors) (Utilities|Array|Get(acopy) _order _array_index))))) (Class|SpiceTypes|FormatRADec (.RA (Utilities|Struct|BreakStateVector_STRUCT (Utilities|Array|Get(acopy) (Variables|Default|GetState%20Vectors) (Utilities|Array|Get(acopy) _order _array_index)))) (.Dec (Utilities|Struct|BreakStateVector_STRUCT (Utilities|Array|Get(acopy) (Variables|Default|GetState%20Vectors) (Utilities|Array|Get(acopy) _order _array_index)))) ", ")))))
        (:Error
          (Development|PrintString _errormessage_2 true true "(R=1.000000,G=0.000000,B=0.000000,A=1.000000)" 3e+01))))
    (:Error
      (Development|PrintString _errormessage true true "(R=1.000000,G=0.000000,B=0.000000,A=1.000000)" 3e+01))))

(event Collision|EventActorBeginOverlap
  (params (OtherActor :type Actor%20Object%20Reference)))

(event EventTick
  (params (DeltaSeconds :type Float%20%28single-precision%29)))

(fn ConstructionScript)

(fn RowtoOrbitalElements
  (params (Row :type Small%20Body%20Record%20STRUCT%20Structure%20%28by%20ref%29) (GM :type S%20Mass%20Constant%20Structure))
  (bind (_spkid _full_name _neo _pha _epoch _e _q _i _om _w _ma) (Utilities|Struct|BreakSmallBodyRecord_STRUCT Row))
  (Utilities|FlowControl|Sequence
    (:then_0
      (bind _out_value (Class|Spice|Convrt _q "AU" "KILOMETERS")
        (:Error
          (Development|PrintString "Error computing conic" true true "(R=1.000000,G=0.000000,B=0.038177,A=1.000000)" :!label _label))))
    (:then_1
      (bind _out_value_2 (Class|Spice|Convrt _i "DEGREES" "RADIANS")
        (:Error
          (goto _label))))
    (:then_2
      (bind _out_value_3 (Class|Spice|Convrt _om "DEGREES" "RADIANS")
        (:Error
          (goto _label))))
    (:then_3
      (bind _out_value_4 (Class|Spice|Convrt _w "DEGREES" "RADIANS")
        (:Error
          (goto _label))))
    (:then_4
      (bind _out_value_5 (Class|Spice|Convrt _ma "DEGREES" "RADIANS")
        (:Error
          (goto _label))))
    (:then_5
      (bind _out (Class|Spice|Unitim _epoch "JDTDB" "ET")
        (:Error
          (goto _label))))
    (:then_6
      _))
  (return (Utilities|Struct|MakeSConicElements (Class|SpiceTypes|ToSDistance(Float) _out_value) _e (Class|SpiceTypes|ToSAngle(Float) _out_value_2) (Class|SpiceTypes|ToSAngle(Float) _out_value_3) (Class|SpiceTypes|ToSAngle(Float) _out_value_4) (Class|SpiceTypes|ToSAngle(Float) _out_value_5) (Class|SpiceTypes|ToSEphemerisTime(Float) _out) GM)))