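; Blueprint function library of example and test routines for the SPICE toolkit.
; Examples propagate Hubble from TLEs with SGP4, read Phobos DSK plates into Unreal mesh buffers, and check orbits after 1 km/s changes to the Moon's velocity.
; Test functions exercise Bodvrd, Bodvcd and Gdpool K2 nodes across output types and bad inputs.
; SPK writing is unfinished: only kernel loading is wired to its entry.
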(fn WritetoSPK
  ;[1 1 1] SPK Writes don't currently work, it's an in-progress feature.
  (Class|Spice|FurnshList (LocalVariables|GetKernels)))

(fn TwoLineElements
  (Utilities|FlowControl|Sequence
    (:then_0
      (Class|Spice|FurnshList (LocalVariables|GetKernels)))
    (:then_1
      ;[1 1 1] Hubble 31 December 2021 20:16:43
      (bind (_errormessage _epoch _elems) (Class|Spice|Getelm "1 20580U 90037B   21365.84494733  .00001067  00000-0  53234-4 0  9998" "2 20580  28.4687 198.7743 0002740  31.8561  96.8389 15.09917499540857")
        (:Success
          (LocalVariables|SetTLE%20Epoch _epoch)
          (LocalVariables|SetTLE%20Elems _elems))))
    (:then_2
      (bind _state (Class|Spice|Evsgp4 (Class|Spice|EtNow) (Class|Spice|Getgeophs "EARTH") (LocalVariables|GetTLE%20Elems))
        (:Success
          (bind _xform (Class|Spice|Sxform (Class|Spice|EtNow) "J2000" "IAU_EARTH")
            (:Success
              (bind _out (Class|Spice|Xfmsta (Class|SpiceTypes|ToSDimensionlessStateVector(SStateVector) (Class|Spice|MxvState _xform _state)) "RECTANGULAR" "PLANETOGRAPHIC" "399")
                (:Success
                  (Development|PrintText 0 (Utilities|Text|FormatText "Hubble {vec}" (Class|SpiceTypes|ToString(SPlanetographicVector) (.r (Utilities|Struct|BreakSPlanetographicStateVector (Class|SpiceTypes|ToSPlanetographicStateVector(SDimensionlessStateVector) _out)))))))))))))))

(fn PhobosLowLevelDSK
  (Utilities|FlowControl|Sequence
    (:then_0
      (Class|Spice|Furnsh "Content/Spice/SImple/Phobos512.bds"
        (:Error
          (Development|PrintString 0 "Requires Phobox512.bds - see commends in FurtherExamples_BPL/Phobos" true true "(R=1.000000,G=0.000000,B=0.000000,A=1.000000)"))))
    (:then_1
      (bind (_errormessage _bodids) (Class|Spice|Dskobj "Content/Spice/Simple/phobos512.bds")
        (:Success
          (for _array_element _bodids
            (LocalVariables|Setbodyid _array_element)
            (Utilities|FlowControl|Sequence
              (:then_0
                (Development|PrintText 0 (Utilities|Text|FormatText "Phobos found body id {id}" (LocalVariables|Getbodyid))))
              (:then_1
                (bind (_errormessage_2 _srfids) (Class|Spice|Dsksrf "Content/Spice/Simple/phobos/phobos512.bds" (LocalVariables|Getbodyid))
                  (:Success
                    (for _array_element_2 _srfids
                      (Development|PrintText 0 (Utilities|Text|FormatText "Phobos body {body} found surface id {id}" (LocalVariables|Getbodyid) _array_element_2))))
                  (:Error
                    (Development|PrintString 0 _errormessage_2 true true "(R=1.000000,G=0.000000,B=0.000000,A=1.000000)"))))))
          ;[1 1 1] Open the dsk file for reading, find the first section
          (bind (_errormessage_3 _handle) (Class|Spice|Dasopr "Content/Spice/Simple/phobos512.bds")
            (:Success
              (bind _output_get (LocalVariables|Sethandle _handle))
              (bind _dladsc (Class|Spice|Dlabfs _output_get)
                (:Found
                  (bind _output_get_2 (LocalVariables|SetDLADescriptor _dladsc))
                  (Utilities|FlowControl|Sequence
                    (:then_0
                      ;[1 1 1] Get the vertex and "plate" counts, size our arrays appropriately
                      (bind (_errormessage_4 _nv _np) (Class|Spice|Dskz02 (LocalVariables|Gethandle) _output_get_2)
                        (:Success
                          (Utilities|Array|Resize (LocalVariables|Getverts) _nv)
                          (Utilities|Array|Resize (LocalVariables|Getnorms) _nv)
                          (Utilities|Array|Resize (LocalVariables|Gettris) (* _np 3))
                          (Development|PrintText 0 (Utilities|Text|FormatText "dskz found Nv {nv} Np {np}" _nv _np)))
                        (:Error
                          (Development|PrintString 0 _errormessage_4 true true "(R=1.000000,G=0.000000,B=0.000000,A=1.000000)"))))
                    (:then_1
                      ;[1 1 1] Fill the local vertex & index buffers with spice data
                      (bind (_errormessage_5 _vrtces) (Class|Spice|Dskv02 (LocalVariables|Gethandle) (LocalVariables|GetDLADescriptor) _nv 1)
                        (:Error
                          (Development|PrintString 0 _errormessage_5 true true "(R=1.000000,G=0.000000,B=0.000000,A=1.000000)"))))
                    (:then_2
                      (bind (_errormessage_6 _plates) (Class|Spice|Dskp02 (LocalVariables|Gethandle) (LocalVariables|GetDLADescriptor) _np 1)
                        (:Error
                          (Development|PrintString 0 _errormessage_6 true true "(R=1.000000,G=0.000000,B=0.000000,A=1.000000)"))))
                    (:then_3
                      ;[1 1 1] Transform the RHS Spice vectors into LHS Unreal Engine Space and save.  Same for vertex normals
                      (for (_ _array_index) _vrtces
                        (bind _normal (Class|Spice|Dskn02 (LocalVariables|Gethandle) (LocalVariables|GetDLADescriptor) _array_index)
                          (:Success
                            (Utilities|Array|SetArrayElem (LocalVariables|Getnorms) _array_index (Class|SpiceTypes|ToVector(SDimensionless) _normal))
                            (Utilities|Array|SetArrayElem (LocalVariables|Getverts) _array_index (Class|SpiceTypes|ToVector(SDistanceVector) (Utilities|Array|Get(acopy) _vrtces _array_index)))))))
                    (:then_4
                      ;[1 1 1] Copy all the indices to the index buffer
                      (for (_array_element_3 _array_index_2) _plates
                        (Utilities|Array|SetArrayElem (LocalVariables|Gettris) (* _array_index_2 3) (.i0 (Utilities|Struct|BreakSPlateIndices _array_element_3)))
                        (Utilities|Array|SetArrayElem (LocalVariables|Gettris) (+ (* _array_index_2 3) 1) (.i1 (Utilities|Struct|BreakSPlateIndices _array_element_3)))
                        (Utilities|Array|SetArrayElem (LocalVariables|Gettris) (+ (+ (* _array_index_2 3) 1) 1) (.i2 (Utilities|Struct|BreakSPlateIndices _array_element_3)))
                        (Class|Spice|Dascls (LocalVariables|Gethandle))
                        (return (LocalVariables|Getverts) (LocalVariables|Gettris) (LocalVariables|Getnorms))))))))
            (:Error
              (Development|PrintString 0 _errormessage_3 true true "(R=1.000000,G=0.000000,B=0.000000,A=1.000000)"))))
        (:Error
          (Development|PrintString 0 _errormessage true true "(R=1.000000,G=0.000000,B=0.000000,A=1.000000)"))))))

(fn TestBodvrdK2Node
  (Utilities|FlowControl|Sequence
    (:then_0
      (Class|Spice|InitAll)
      (bind _errormessage (Class|Spice|FurnshList (LocalVariables|GetKernels))
        (:Success
          (bind _errormessage_2 (|Bodvrd "All" "EARTH" "GM")
            (:Success
              (bind _errormessage_3 (|Bodvrd "All" "EARTH" "RADII")
                (:Success
                  (bind _errormessage_4 (|Bodvrd "All" "EARTH" "RADII")
                    (:Success
                      (|Bodvrd "All" "EARTH" "RADII"
                        (:Success
                          (Development|PrintString 0 "Should see this")
                          (|Bodvrd "All" "EARTH" "RADII"))))
                    (:Error
                      (Development|PrintString 0 _errormessage_4 true true "(R=1.000000,G=0.000000,B=0.000000,A=1.000000)"))))
                (:Error
                  (Development|PrintString 0 _errormessage_3 true true "(R=1.000000,G=0.000000,B=0.000000,A=1.000000)"))))
            (:Error
              (Development|PrintString 0 _errormessage_2 true true "(R=1.000000,G=0.000000,B=0.000000,A=1.000000)"))))
        (:Error
          (Development|PrintString 0 _errormessage true true "(R=1.000000,G=0.000000,B=0.000000,A=1.000000)"))))
    (:then_1
      (bind (_value _errormessage_5) (|Bodvrd "All" "EARTH" "GM")
        (:Success
          (LocalVariables|SetDouble _value)
          (bind (_value_2 _errormessage_6) (|Bodvrd "All" "EARTH" "GM222")
            (:Success
              (LocalVariables|SetDouble _value_2))
            (:Error
              (Development|PrintString 0 _errormessage_6 true true "(R=1.000000,G=0.000000,B=0.000000,A=1.000000)"))))
        (:Error
          (Development|PrintString 0 _errormessage_5 true true "(R=1.000000,G=0.000000,B=0.000000,A=1.000000)"))))
    (:then_2
      (bind (_value_3 _errormessage_7) (|Bodvrd "All" "EARTH" "RADII")
        (:Success
          (LocalVariables|SetDouble%20Array _value_3)
          (bind (_value_4 _errormessage_8) (|Bodvrd "All" "EARTH" "RADII222")
            (:Success
              (LocalVariables|SetDouble%20Array _value_4))
            (:Error
              (Development|PrintString 0 _errormessage_8 true true "(R=1.000000,G=0.000000,B=0.000000,A=1.000000)"))))
        (:Error
          (Development|PrintString 0 _errormessage_7 true true "(R=1.000000,G=0.000000,B=0.000000,A=1.000000)"))))
    (:then_3
      (bind (_value_5 _errormessage_9) (|Bodvrd "All" "EARTH" "RADII")
        (:Success
          (LocalVariables|SetSDimensionlessVector _value_5)
          (bind (_value_6 _errormessage_10) (|Bodvrd "All" "sdf" "sdfas")
            (:Success
              (LocalVariables|SetSDimensionlessVector _value_6))
            (:Error
              (Development|PrintString 0 _errormessage_10 true true "(R=1.000000,G=0.000000,B=0.000000,A=1.000000)"))))
        (:Error
          (Development|PrintString 0 _errormessage_9 true true "(R=1.000000,G=0.000000,B=0.000000,A=1.000000)"))))
    (:then_4
      (bind (_value_7 _errormessage_11) (|Bodvrd "All" "EARTH" "GM")
        (:Success
          (LocalVariables|SetSMassConstant _value_7)
          (bind (_value_8 _errormessage_12) (|Bodvrd "All" "" "RADII")
            (:Success
              (LocalVariables|SetSMassConstant _value_8))
            (:Error
              (Development|PrintString 0 _errormessage_12 true true "(R=1.000000,G=0.000000,B=0.000000,A=1.000000)"))))
        (:Error
          (Development|PrintString 0 _errormessage_11 true true "(R=1.000000,G=0.000000,B=0.000000,A=1.000000)"))))
    (:then_5
      (bind (_value_9 _errormessage_13) (|Bodvrd "All" "EARTH" "GM")
        (:Success
          (LocalVariables|SetSDistance _value_9)
          (bind (_value_10 _errormessage_14) (|Bodvrd "All" "EARTH")
            (:Success
              (LocalVariables|SetSDistance _value_10))
            (:Error
              (Development|PrintString 0 _errormessage_14 true true "(R=1.000000,G=0.000000,B=0.000000,A=1.000000)"))))
        (:Error
          (Development|PrintString 0 _errormessage_13 true true "(R=1.000000,G=0.000000,B=0.000000,A=1.000000)"))))
    (:then_6
      (bind (_value_11 _errormessage_15) (|Bodvrd "All" "EARTH" "GM")
        (:Success
          (LocalVariables|SetSAngle _value_11)
          (bind (_value_12 _errormessage_16) (|Bodvrd "All")
            (:Success
              (LocalVariables|SetSAngle _value_12))
            (:Error
              (Development|PrintString 0 _errormessage_16 true true "(R=1.000000,G=0.000000,B=0.000000,A=1.000000)"))))
        (:Error
          (Development|PrintString 0 _errormessage_15 true true "(R=1.000000,G=0.000000,B=0.000000,A=1.000000)"))))
    (:then_7
      (bind (_value_13 _errormessage_17) (|Bodvrd "All" "EARTH" "RADII")
        (:Success
          (LocalVariables|SetSDistanceVector _value_13)
          (bind (_value_14 _errormessage_18) (|Bodvrd "All" "EARTH" "EARTH")
            (:Success
              (LocalVariables|SetSDistanceVector _value_14))
            (:Error
              (Development|PrintString 0 _errormessage_18 true true "(R=1.000000,G=0.000000,B=0.000000,A=1.000000)"))))
        (:Error
          (Development|PrintString 0 _errormessage_17 true true "(R=1.000000,G=0.000000,B=0.000000,A=1.000000)"))))
    (:then_8
      (bind (_value_15 _errormessage_19) (|Bodvrd "All" "EARTH" "RADII")
        (:Success
          (LocalVariables|SetSVelocityVector _value_15)
          (bind (_value_16 _errormessage_20) (|Bodvrd "All" "RADII" "RADII")
            (:Success
              (LocalVariables|SetSDistanceVector _value_16))
            (:Error
              (Development|PrintString 0 _errormessage_20 true true "(R=1.000000,G=0.000000,B=0.000000,A=1.000000)"))))
        (:Error
          (Development|PrintString 0 _errormessage_19 true true "(R=1.000000,G=0.000000,B=0.000000,A=1.000000)"))))
    (:then_9
      (Development|PrintString 0 (Utilities|String|ToString(Float) (LocalVariables|GetDouble)))
      (Development|PrintString 0 (Class|SpiceTypes|ToString(SDimensionlessVector) (LocalVariables|GetSDimensionlessVector)))
      (Development|PrintString 0 (Class|SpiceTypes|ToString(SMassConstant) (LocalVariables|GetSMassConstant)))
      (Development|PrintString 0 (Class|SpiceTypes|ToString(SDistance) (LocalVariables|GetSDistance)))
      (Development|PrintString 0 (Class|SpiceTypes|ToString(SAngle) (LocalVariables|GetSAngle)))
      (Development|PrintString 0 (Class|SpiceTypes|ToString(SDistanceVector) (LocalVariables|GetSDistanceVector)))
      (Development|PrintString 0 (Class|SpiceTypes|ToString(SVelocityVector) (LocalVariables|GetSVelocityVector)))
      (bind (_value_17 _errormessage_21) (|Bodvrd "All" (LocalVariables|GetBody) (LocalVariables|GetItem))
        (:Success
          (Development|PrintString 0 (Class|SpiceTypes|ToString(SMassConstant) _value_17)))
        (:Error
          (Development|PrintString 0 _errormessage_21 true true "(R=1.000000,G=0.000000,B=0.000000,A=1.000000)"))))))

(fn TestBodvcdK2Node
  (Utilities|FlowControl|Sequence
    (:then_0
      (Class|Spice|InitAll)
      (bind _errormessage (Class|Spice|FurnshList (LocalVariables|GetKernels))
        (:Success
          (bind _errormessage_2 (|Bodvcd "All" 399 "GM")
            (:Success
              (bind _errormessage_3 (|Bodvcd "All" 399 "RADII")
                (:Success
                  (bind _errormessage_4 (|Bodvcd "All" 399 "RADII")
                    (:Success
                      (|Bodvcd "All" 399 "RADII"
                        (:Success
                          (Development|PrintString 0 "Should see this")
                          (|Bodvcd "All" 399 "RADII"))))
                    (:Error
                      (Development|PrintString 0 _errormessage_4 true true "(R=1.000000,G=0.000000,B=0.000000,A=1.000000)"))))
                (:Error
                  (Development|PrintString 0 _errormessage_3 true true "(R=1.000000,G=0.000000,B=0.000000,A=1.000000)"))))
            (:Error
              (Development|PrintString 0 _errormessage_2 true true "(R=1.000000,G=0.000000,B=0.000000,A=1.000000)"))))
        (:Error
          (Development|PrintString 0 _errormessage true true "(R=1.000000,G=0.000000,B=0.000000,A=1.000000)"))))
    (:then_1
      (bind (_value _errormessage_5) (|Bodvcd "All" 399 "GM")
        (:Success
          (LocalVariables|SetDouble _value)
          (bind (_value_2 _errormessage_6) (|Bodvcd "All" 399 "GM222")
            (:Success
              (LocalVariables|SetDouble _value_2))
            (:Error
              (Development|PrintString 0 _errormessage_6 true true "(R=1.000000,G=0.000000,B=0.000000,A=1.000000)"))))
        (:Error
          (Development|PrintString 0 _errormessage_5 true true "(R=1.000000,G=0.000000,B=0.000000,A=1.000000)"))))
    (:then_2
      (bind (_value_3 _errormessage_7) (|Bodvcd "All" 399 "GM")
        (:Success
          (LocalVariables|SetDouble%20Array _value_3)
          (bind (_value_4 _errormessage_8) (|Bodvcd "All" 399 "RRRRR")
            (:Success
              (LocalVariables|SetDouble%20Array _value_4))
            (:Error
              (Development|PrintString 0 _errormessage_8 true true "(R=1.000000,G=0.000000,B=0.000000,A=1.000000)"))))
        (:Error
          (Development|PrintString 0 _errormessage_7 true true "(R=1.000000,G=0.000000,B=0.000000,A=1.000000)"))))
    (:then_3
      (bind (_value_5 _errormessage_9) (|Bodvcd "All" 399 "RADII")
        (:Success
          (LocalVariables|SetSDimensionlessVector _value_5)
          (bind (_value_6 _errormessage_10) (|Bodvcd "All" 222 "RRRRR")
            (:Success
              (LocalVariables|SetSDimensionlessVector _value_6))
            (:Error
              (Development|PrintString 0 _errormessage_10 true true "(R=1.000000,G=0.000000,B=0.000000,A=1.000000)"))))
        (:Error
          (Development|PrintString 0 _errormessage_9 true true "(R=1.000000,G=0.000000,B=0.000000,A=1.000000)"))))
    (:then_4
      (bind (_value_7 _errormessage_11) (|Bodvcd "All" 399 "GM")
        (:Success
          (LocalVariables|SetSMassConstant _value_7)
          (bind (_value_8 _errormessage_12) (|Bodvcd "All" 0 "RADII")
            (:Success
              (LocalVariables|SetSMassConstant _value_8))
            (:Error
              (Development|PrintString 0 _errormessage_12 true true "(R=1.000000,G=0.000000,B=0.000000,A=1.000000)"))))
        (:Error
          (Development|PrintString 0 _errormessage_11 true true "(R=1.000000,G=0.000000,B=0.000000,A=1.000000)"))))
    (:then_5
      (bind (_value_9 _errormessage_13) (|Bodvcd "All" 399 "GM")
        (:Success
          (LocalVariables|SetSDistance _value_9)
          (bind (_value_10 _errormessage_14) (|Bodvcd "All" 399)
            (:Success
              (LocalVariables|SetSDistance _value_10))
            (:Error
              (Development|PrintString 0 _errormessage_14 true true "(R=1.000000,G=0.000000,B=0.000000,A=1.000000)"))))
        (:Error
          (Development|PrintString 0 _errormessage_13 true true "(R=1.000000,G=0.000000,B=0.000000,A=1.000000)"))))
    (:then_6
      (bind (_value_11 _errormessage_15) (|Bodvcd "All" 399 "GM")
        (:Success
          (LocalVariables|SetSAngle _value_11)
          (bind (_value_12 _errormessage_16) (|Bodvcd "All")
            (:Success
              (LocalVariables|SetSAngle _value_12))
            (:Error
              (Development|PrintString 0 _errormessage_16 true true "(R=1.000000,G=0.000000,B=0.000000,A=1.000000)"))))
        (:Error
          (Development|PrintString 0 _errormessage_15 true true "(R=1.000000,G=0.000000,B=0.000000,A=1.000000)"))))
    (:then_7
      (bind (_value_13 _errormessage_17) (|Bodvcd "All" 399 "RADII")
        (:Success
          (LocalVariables|SetSDistanceVector _value_13)
          (bind (_value_14 _errormessage_18) (|Bodvrd "All" "EARTH" "EARTH")
            (:Success
              (LocalVariables|SetSDistanceVector _value_14))
            (:Error
              (Development|PrintString 0 _errormessage_18 true true "(R=1.000000,G=0.000000,B=0.000000,A=1.000000)"))))
        (:Error
          (Development|PrintString 0 _errormessage_17 true true "(R=1.000000,G=0.000000,B=0.000000,A=1.000000)"))))
    (:then_8
      (bind (_value_15 _errormessage_19) (|Bodvcd "All" 399 "RADII")
        (:Success
          (LocalVariables|SetSVelocityVector _value_15)
          (bind (_value_16 _errormessage_20) (|Bodvrd "All" "RADII" "RADII")
            (:Success
              (LocalVariables|SetSDistanceVector _value_16))
            (:Error
              (Development|PrintString 0 _errormessage_20 true true "(R=1.000000,G=0.000000,B=0.000000,A=1.000000)"))))
        (:Error
          (Development|PrintString 0 _errormessage_19 true true "(R=1.000000,G=0.000000,B=0.000000,A=1.000000)"))))
    (:then_9
      (Development|PrintString 0 (Utilities|String|ToString(Float) (LocalVariables|GetDouble)))
      (Development|PrintString 0 (Class|SpiceTypes|ToString(SDimensionlessVector) (LocalVariables|GetSDimensionlessVector)))
      (Development|PrintString 0 (Class|SpiceTypes|ToString(SMassConstant) (LocalVariables|GetSMassConstant)))
      (Development|PrintString 0 (Class|SpiceTypes|ToString(SDistance) (LocalVariables|GetSDistance)))
      (Development|PrintString 0 (Class|SpiceTypes|ToString(SAngle) (LocalVariables|GetSAngle)))
      (Development|PrintString 0 (Class|SpiceTypes|ToString(SDistanceVector) (LocalVariables|GetSDistanceVector)))
      (Development|PrintString 0 (Class|SpiceTypes|ToString(SVelocityVector) (LocalVariables|GetSVelocityVector)))
      (bind (_value_17 _errormessage_21) (|Bodvcd "All" (LocalVariables|GetBody) (LocalVariables|GetItem))
        (:Success
          (Development|PrintString 0 (Class|SpiceTypes|ToString(SMassConstant) _value_17)))
        (:Error
          (Development|PrintString 0 _errormessage_21 true true "(R=1.000000,G=0.000000,B=0.000000,A=1.000000)"))))))

(fn TestGdpoolK2Node
  (Utilities|FlowControl|Sequence
    (:then_0
      (Class|Spice|InitAll)
      (bind _errormessage (Class|Spice|FurnshList (LocalVariables|GetKernels))
        (:Success
          (|Gdpool "All" "DTEST_VAL"
            (:Success
              (|Gdpool "All" "DTEST_VAL"
                (:Success
                  (|Gdpool "All" "DTEST_VAL"
                    (:Success
                      (|Gdpool "All" "DTEST_VAL"
                        (:Success
                          (Development|PrintString 0 "Should see this")
                          (|Gdpool "All" "DTEST_VAL"))))
                    (:Error
                      (Development|PrintString 0 "DTEST_VAL Not Found" true true "(R=1.000000,G=0.000000,B=0.000000,A=1.000000)"))))
                (:Error
                  (Development|PrintString 0 "DTEST_VAL Not Found" true true "(R=1.000000,G=0.000000,B=0.000000,A=1.000000)"))))
            (:Error
              (Development|PrintString 0 "DTEST_VAL Not Found" true true "(R=1.000000,G=0.000000,B=0.000000,A=1.000000)"))))
        (:Error
          (Development|PrintString 0 _errormessage true true "(R=1.000000,G=0.000000,B=0.000000,A=1.000000)"))))
    (:then_1
      (bind _value (|Gdpool "All" "DTEST_VAL")
        (:Success
          (LocalVariables|SetDouble _value)
          (bind _value_2 (|Gdpool "All" "NTEST_VAL")
            (:Success
              (LocalVariables|SetDouble _value_2)
              (Development|PrintString 0 "Bad Value Found" true true "(R=1.000000,G=0.000000,B=0.000000,A=1.000000)"))))
        (:Error
          (Development|PrintString 0 "Value Not Found" true true "(R=1.000000,G=0.000000,B=0.000000,A=1.000000)"))))
    (:then_2
      (bind _value_3 (|Gdpool "All" "ATEST_VAL")
        (:Success
          (LocalVariables|SetDouble%20Array _value_3)
          (bind _value_4 (|Gdpool "All" "BTEST_VAL")
            (:Success
              (LocalVariables|SetDouble%20Array _value_4)
              (Development|PrintString 0 "Bad Value Found" true true "(R=1.000000,G=0.000000,B=0.000000,A=1.000000)"))))
        (:Error
          (Development|PrintString 0 "Value Not Found" true true "(R=1.000000,G=0.000000,B=0.000000,A=1.000000)"))))
    (:then_3
      (bind _value_5 (|Gdpool "All" "DTEST_VAL")
        (:Success
          (LocalVariables|SetSDimensionlessVector _value_5)
          (bind _value_6 (|Gdpool "All" "CTEST_VAL")
            (:Success
              (LocalVariables|SetSDimensionlessVector _value_6)
              (Development|PrintString 0 "Bad Value Found" true true "(R=1.000000,G=0.000000,B=0.000000,A=1.000000)"))))
        (:Error
          (Development|PrintString 0 "Value Not Found" true true "(R=1.000000,G=0.000000,B=0.000000,A=1.000000)"))))
    (:then_4
      (bind _value_7 (|Gdpool "All" "DTEST_VAL")
        (:Success
          (LocalVariables|SetSMassConstant _value_7)
          (bind _value_8 (|Gdpool "All")
            (:Success
              (LocalVariables|SetSMassConstant _value_8)
              (Development|PrintString 0 "Bad Value Found" true true "(R=1.000000,G=0.000000,B=0.000000,A=1.000000)"))))
        (:Error
          (Development|PrintString 0 "Value Not Found" true true "(R=1.000000,G=0.000000,B=0.000000,A=1.000000)"))))
    (:then_5
      (bind _value_9 (|Gdpool "All" "DTEST_VAL")
        (:Success
          (LocalVariables|SetSDistance _value_9)
          (bind _value_10 (|Gdpool "All" "FOO")
            (:Success
              (LocalVariables|SetSDistance _value_10)
              (Development|PrintString 0 "Bad Value Found" true true "(R=1.000000,G=0.000000,B=0.000000,A=1.000000)"))))
        (:Error
          (Development|PrintString 0 "Value Not Found" true true "(R=1.000000,G=0.000000,B=0.000000,A=1.000000)"))))
    (:then_6
      (bind _value_11 (|Gdpool "All" "DTEST_VAL")
        (:Success
          (LocalVariables|SetSAngle _value_11)
          (bind _value_12 (|Gdpool "All" "FOO")
            (:Success
              (LocalVariables|SetSAngle _value_12)
              (Development|PrintString 0 "Bad Value Found" true true "(R=1.000000,G=0.000000,B=0.000000,A=1.000000)"))))
        (:Error
          (Development|PrintString 0 "Value Not Found" true true "(R=1.000000,G=0.000000,B=0.000000,A=1.000000)"))))
    (:then_7
      (bind _value_13 (|Gdpool "All" "DTEST_VAL")
        (:Success
          (LocalVariables|SetSDistanceVector _value_13)
          (bind _value_14 (|Gdpool "All" "FOO")
            (:Success
              (LocalVariables|SetSDistanceVector _value_14)
              (Development|PrintString 0 "Bad Value Found" true true "(R=1.000000,G=0.000000,B=0.000000,A=1.000000)"))))
        (:Error
          (Development|PrintString 0 "Value Not Found" true true "(R=1.000000,G=0.000000,B=0.000000,A=1.000000)"))))
    (:then_8
      (bind _value_15 (|Gdpool "All" "DTEST_VAL")
        (:Success
          (LocalVariables|SetSVelocityVector _value_15)
          (bind _value_16 (|Gdpool "All" "S_TEST_VAL")
            (:Success
              (LocalVariables|SetSVelocityVector _value_16)
              (Development|PrintString 0 "Bad Value Found" true true "(R=1.000000,G=0.000000,B=0.000000,A=1.000000)"))))
        (:Error
          (Development|PrintString 0 "Value Not Found" true true "(R=1.000000,G=0.000000,B=0.000000,A=1.000000)"))))
    (:then_9
      (Development|PrintString 0 (Utilities|String|ToString(Float) (LocalVariables|GetDouble)))
      (Development|PrintString 0 (Class|SpiceTypes|ToString(SDimensionlessVector) (LocalVariables|GetSDimensionlessVector)))
      (Development|PrintString 0 (Class|SpiceTypes|ToString(SMassConstant) (LocalVariables|GetSMassConstant)))
      (Development|PrintString 0 (Class|SpiceTypes|ToString(SDistance) (LocalVariables|GetSDistance)))
      (Development|PrintString 0 (Class|SpiceTypes|ToString(SAngle) (LocalVariables|GetSAngle)))
      (Development|PrintString 0 (Class|SpiceTypes|ToString(SDistanceVector) (LocalVariables|GetSDistanceVector)))
      (Development|PrintString 0 (Class|SpiceTypes|ToString(SVelocityVector) (LocalVariables|GetSVelocityVector)))
      (bind _value_17 (|Gdpool "All" (LocalVariables|Getname))
        (:Success
          (Development|PrintString 0 (Class|SpiceTypes|ToString(SMassConstant) _value_17)))
        (:Error
          (Development|PrintString 0 "Value Not Found" true true "(R=1.000000,G=0.000000,B=0.000000,A=1.000000)"))))))

(fn CollisionwithMoon
  (Utilities|FlowControl|Sequence
    (:then_0
      (bind _errormessage (Class|Spice|FurnshList (LocalVariables|GetRequired%20Kernels))
        (:Success
          (bind _value (|Bodvrd "All" "EARTH" "RADII")
            (:Success
              (LocalVariables|SetEARTH_Re (.x (Utilities|Struct|BreakSDistanceVector _value)))
              (bind _value_2 (|Bodvrd "All" "MOON" "RADII")
                (:Success
                  (LocalVariables|SetMOON_Re (.x (Utilities|Struct|BreakSDistanceVector _value_2))))))))
        (:Error
          (Development|PrintString 0 _errormessage true true "(R=1.000000,G=0.000000,B=0.000000,A=1.000000)" 3e+01))))
    (:then_1
      (bind _value_3 (|Bodvrd "All" "EARTH" "GM")
        (:Success
          (LocalVariables|SetGM _value_3))))
    (:then_2
      ;[1 1 1] So... where's the moon right now?
      (bind _state (Class|Spice|Spkezr (Class|Spice|EtNow) "MOON" "EARTH BARYCENTER" "ECLIPJ2000" "None")
        (:Success
          ;[1 1 1] Get New Orbital Elements afor the prograde case
          (bind _elts (Class|Spice|Oscelt (Utilities|Struct|MakeSStateVector (.r (Utilities|Struct|BreakSStateVector _state)) (+ (.v (Utilities|Struct|BreakSStateVector _state)) (Class|SpiceTypes|ToSVelocityVector(SDimensionlessVector) (Class|Spice|VhatVelocity (.v (Utilities|Struct|BreakSStateVector _state)))))) (Class|Spice|EtNow) (LocalVariables|GetGM))
            (:Success
              (Development|PrintString 0 (Class|SpiceTypes|ToString(SConicElements) _elts) true true "(R=0.000000,G=0.660000,B=1.000000,A=1.000000)" 3e+01)
              ;[1 1 1] See of the moon's on an escape trajectory (e > 1)
              (if (> (.Eccentricity (Utilities|Struct|BreakSConicElements _elts)) 1.0)
                (Development|PrintString 0 "Uh"))
              ;[1 1 1] Get New Orbital Elements for the retrograde case
              (bind _elts_2 (Class|Spice|Oscelt (Utilities|Struct|MakeSStateVector (.r (Utilities|Struct|BreakSStateVector _state)) (- (.v (Utilities|Struct|BreakSStateVector _state)) (Class|SpiceTypes|ToSVelocityVector(SDimensionlessVector) (Class|Spice|VhatVelocity (.v (Utilities|Struct|BreakSStateVector _state)))))) (Class|Spice|EtNow) (LocalVariables|GetGM))
                (:Success
                  (Development|PrintString 0 (Class|SpiceTypes|ToString(SConicElements) _elts_2) true true "(R=0.000000,G=0.298049,B=1.000000,A=1.000000)" 3e+01)
                  ;[1 1 1] See if the Moon's coming close enough to the earth, in theory, it collides
                  (if (< (Class|SpiceTypes|ToFloat(SDistance) (.PerifocalDistance (Utilities|Struct|BreakSConicElements _elts_2))) (Class|SpiceTypes|ToFloat(SDistance) (+ (LocalVariables|GetEARTH_Re) (LocalVariables|GetMOON_Re))))
                    (Development|PrintString 0)))))))))))