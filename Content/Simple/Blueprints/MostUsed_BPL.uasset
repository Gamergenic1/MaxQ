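; Blueprint function library porting NAIF's "Most Used" CSPICE examples to SPICE Blueprint nodes, one function per topic.
; Implemented examples load kernels via Furnsh or FurnshList, run time, frame, ephemeris, instrument, coordinate, illumination or orbital-element queries, and print results, mostly with error branches.
; DSK and surface-name topics only print "not implemented" notices, and many later topics are empty stubs.
; A ComputeFlattening helper supplies the flattening value omitted from NAIF's coordinates example.
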(fn LoadingandUnloadingSPICEKernels
  ;[0 0 0 1 10] Loading and Unloading SPICE Kernels
  ; APIs:
  ; furnsh_c - loads an individual kernel or a collection of kernels.
  ; unload_c - unloads an individual kernel or a collection of kernels.
  ; Brief Example:
  ;    Generic LSK and PCK files listed in a meta-kernel named
  ;    "mykernels.furnsh" and containing
  ;
  ;       \begindata
  ;          KERNELS_TO_LOAD = (
  ;                             '/kernels/gen/lsk/naif0008.tls'
  ;                             '/kernels/gen/pck/pck00008.tps'
  ;                            )
  ;       \begintext
  ;
  ;    are loaded with a single call to furnsh_c:
  ;
  ;       furnsh_c ( "mykernels.furnsh" );
  ; Reference documents:
  ; kernel.req - reference on loading/unloading kernels and text kernel format
  ;
  ; https://naif.jpl.nasa.gov/pub/naif/toolkit_docs/C/info/mostused.html#A
  ;[1 1 1] Space Toolkit Alternative #2 : Load from a pre-filled list
  (bind _errormessage (Class|Spice|FurnshList (LocalVariables|GetKernel%20Files%20To%20Load))
    (:Success
      (Development|PrintString 0 "Loading and Unloading SPICE Kernels")
      (for _array_element (LocalVariables|GetKernel%20Files%20To%20Load)
        (bind _errormessage_2 (Class|Spice|Unload _array_element)
          (:Error
            (Development|PrintString 0 _errormessage_2 true true "(R=1.000000,G=0.000000,B=0.000000,A=1.000000)")))))
    (:Error
      (Development|PrintString 0 _errormessage true true "(R=1.000000,G=0.000000,B=0.000000,A=1.000000)"))))

(fn ConvertingBetweenUTCandEphemerisTime(LSK)
  ;[0 0 0 1 10] Converting between UTC and Ephemeris Time (LSK)
  ; APIs:
  ; furnsh_c - loads an individual kernel or a collection of kernels.
  ; str2et_c - converts a time string to ET seconds past J2000.
  ; timout_c - converts ET seconds past J2000 to a time string.
  ; Brief Example:
  ;    The following example loads an LSK file, converts a UTC string to ET
  ;    seconds, adds 1 day and converts TDB seconds back to a UTC string in
  ;    ISO DOY format:
  ;
  ;       SpiceDouble   et;
  ;       SpiceChar     utc[32];
  ;
  ;       /*
  ;          load LSK file
  ;       */
  ;       furnsh_c  ( "naif0008.tls" );
  ;
  ;       /*
  ;          convert UTC to ET
  ;       */
  ;       str2et_c  ( "2005 DEC 31 12:00", &et );
  ;
  ;       /*
  ;          add 1 day to ET and convert it back to UTC
  ;       */
  ;       timout_c ( et+spd_c(), "YYYY-DOYTHR:MN:SC.### ::RND", 32, utc );
  ; Reference documents:
  ; time.req - reference on time systems and conversions supported in SPICE
  ; kernel.req - reference on loading/unloading kernels and text kernel format
  ;
  ; https://naif.jpl.nasa.gov/pub/naif/toolkit_docs/C/info/mostused.html#B
  ;[1 1 1] Example, as given
  (bind _errormessage (Class|Spice|Furnsh "Content/Spice/Simple/naif0008.tls")
    (:Success
      (bind (_errormessage_2 _et) (Class|Spice|Str2et "2005 DEC 31 12:00")
        (:Success
          (bind (_errormessage_3 _output) (Class|Spice|Timout (+ _et (Class|Spice|Spd)) "YYYY-DOYTHR:MN:SC.### ::RND")
            (:Success
              (Development|PrintString 0 (Utilities|String|Append "Converting between UTC and Ephemeris Time (LSK):  " _output)))
            (:Error
              (Development|PrintString 0 _errormessage_3 true true "(R=1.000000,G=0.000000,B=0.000000,A=1.000000)"))))
        (:Error
          (Development|PrintString 0 _errormessage_2 true true "(R=1.000000,G=0.000000,B=0.000000,A=1.000000)"))))
    (:Error
      (Development|PrintString 0 _errormessage true true "(R=1.000000,G=0.000000,B=0.000000,A=1.000000)"))))

(fn ConvertingBetweenEphemerisTimeandSpacecraftClock(SCLK)
  (bind _sclk (LocalVariables|Getsclk))
  (bind _scid (LocalVariables|Getscid))
  ;[0 0 0 1 10] Converting between Ephemeris Time and Spacecraft Clock (SCLK)
  ; APIs:
  ; furnsh_c - loads individual kernels and collections of kernels.
  ; scs2e_c - converts an SCLK string to ET seconds past J2000.
  ; sce2s_c - converts ET seconds past J2000 to SCLK string.
  ; sct2e_c - converts an encoded SCLK to ET seconds past J2000.
  ; sce2c_c - converts ET seconds past J2000 to encoded SCLK.
  ; scencd_c - converts an SCLK string to encoded SCLK.
  ; scdecd_c - converts an encoded SCLK to SCLK string.
  ; Brief Example:
  ;    The following example loads an LSK file and an MGS SCLK file, then
  ;    converts an MGS SCLK string to ET and encoded SCLK:
  ;
  ;       SpiceChar   * sclk;
  ;       SpiceDouble   et;
  ;       SpiceDouble   sclkdp;
  ;       SpiceInt      scid = -94;
  ;
  ;       /*
  ;          load LSK and SCLK files
  ;       */
  ;       furnsh_c ( "naif0008.tls" );
  ;       furnsh_c ( "mgs_sclkscet_00061.tsc" );
  ;
  ;       /*
  ;          convert string SCLK to ET and to encoded SCLK
  ;       */
  ;       sclk = "820584056:121";
  ;       scs2e_c  ( scid, sclk, &et );
  ;       scencd_c ( scid, sclk, &sclkdp );
  ; Reference documents:
  ; sclk.req - reference on on-board clock (SCLK) implementation in SPICE
  ; kernel.req - reference on loading/unloading kernels and text kernel format
  ;
  ; https://naif.jpl.nasa.gov/pub/naif/toolkit_docs/C/info/mostused.html#C
  ;[1 1 1] Example as given
  (Utilities|FlowControl|Sequence
    (:then_0
      (bind _errormessage (Class|Spice|Furnsh "Content/Spice/Simple/naif0008.tls")
        (:Error
          (Development|PrintString 0 _errormessage true true "(R=1.000000,G=0.000000,B=0.000000,A=1.000000)"))))
    (:then_1
      (bind _errormessage_2 (Class|Spice|Furnsh "Content/Spice/Simple/mgs_sclkscet_00061.tsc")
        (:Error
          (Development|PrintString 0 _errormessage_2 true true "(R=1.000000,G=0.000000,B=0.000000,A=1.000000)"))))
    (:then_2
      (bind (_errormessage_3 _et) (Class|Spice|Scs2e _scid _sclk)
        (:Success
          (bind (_errormessage_4 _utcstr) (Class|Spice|Et2utc _et "Calendar")
            (:Success
              (Development|PrintString 0 (Utilities|String|Append "Converting between Ephemeris Time and Spacecraft Clock (SCLK): " _utcstr)))
            (:Error
              (Development|PrintString 0 _errormessage_4 true true "(R=1.000000,G=0.000000,B=0.000000,A=1.000000)"))))
        (:Error
          (Development|PrintString 0 _errormessage_3 true true "(R=1.000000,G=0.000000,B=0.000000,A=1.000000)"))))
    (:then_3
      (bind (_errormessage_5 _sclkdp) (Class|Spice|Scencd _scid _sclk)
        (:Success
          (Development|PrintString 0 (Utilities|String|Append "Converting between Ephemeris Time and Spacecraft Clock (SCLK): " (Utilities|String|ToString(Float) _sclkdp))))
        (:Error
          (Development|PrintString 0 _errormessage_5 true true "(R=1.000000,G=0.000000,B=0.000000,A=1.000000)"))))))

(fn RetrievingConstantsandOrientationforNaturalBodies(PCK)
  ;[0 0 0 1 10] Constants and Orientation for Natural Bodies (PCK)
  ; APIs:
  ; furnsh_c - loads individual kernels and collections of kernels.
  ; bodfnd_c - determines whether values exist for some item for a body in the kernel pool.
  ; bodvrd_c - retrieves from the kernel pool the values of an item associated with a body.
  ; pxform_c - returns the 3x3 matrix rotating a position vector one frame to another.
  ; sxform_c - returns the 6x6 matrix rotating a state vector from one frame to another.
  ; pckfrm_c - finds the set of reference frame class ID codes of all frames in a binary PCK file.
  ; pckcov_c - finds the coverage window for a reference frame in a binary PCK file.
  ; Brief Example:
  ;    The following example retrieves radii for Mars and computes
  ;    orientation of the Mars body-fixed frame:
  ;
  ;       SpiceDouble   et;
  ;       SpiceDouble   mat[3][3];
  ;       SpiceDouble   radii[3];
  ;       SpiceInt      n;
  ;
  ;       /*
  ;          load LSK and PCK files
  ;       */
  ;       furnsh_c ( "naif0008.tls" );
  ;       furnsh_c ( "pck00008.tpc" );
  ;
  ;       /*
  ;          retrieve Mars radii
  ;       */
  ;       bodvrd_c ( "MARS", "RADII", 3, &n, radii );
  ;
  ;       /*
  ;          convert UTC to ET
  ;       */
  ;       str2et_c ( "2005-DEC-28 12:00", &et );
  ;
  ;       /*
  ;          compute Mars orientation relative to the J2000 frame
  ;       */
  ;       pxform_c ( "J2000", "IAU_MARS", et, mat );
  ; Reference documents:
  ; pck.req - reference on Planetary Constants Kernel (PCK) subsystem of SPICE
  ; kernel.req - reference on loading/unloading kernels and text kernel format
  ;
  ; https://naif.jpl.nasa.gov/pub/naif/toolkit_docs/C/info/mostused.html#D
  (Utilities|FlowControl|Sequence
    (:then_0
      ;[1 1 1] Example as given
      (bind _errormessage (Class|Spice|Furnsh "Content/Spice/Simple/naif0008.tls")
        (:Error
          (Development|PrintString 0 _errormessage true true "(R=1.000000,G=0.000000,B=0.000000,A=1.000000)"))))
    (:then_1
      (bind _errormessage_2 (Class|Spice|Furnsh "Content/Spice/Simple/pck00008.tpc")
        (:Error
          (Development|PrintString 0 _errormessage_2 true true "(R=1.000000,G=0.000000,B=0.000000,A=1.000000)"))))
    (:then_2
      (bind (_errormessage_3 _returnvalue) (Class|Spice|BodvrdDistanceVector "MARS" "RADII")
        (:Error
          (Development|PrintString 0 _errormessage_3 true true "(R=1.000000,G=0.000000,B=0.000000,A=1.000000)"))))
    (:then_3
      (bind (_errormessage_4 _et) (Class|Spice|Str2et "2005-DEC-28 12:00")
        (:Success
          (bind _errormessage_5 (Class|Spice|Pxform "J2000" _et "IAU_MARS")
            (:Success
              (Development|PrintString 0 (Utilities|String|ToString(Text) (Utilities|Text|FormatText "Constants and Orientation for Natural Bodies (PCK): Mars radii: ({x} km, {y} km. {z} km)" (.X (Math|Vector|BreakVector (Class|SpiceTypes|ToVector(SDistanceVector) _returnvalue))) (.Y (Math|Vector|BreakVector (Class|SpiceTypes|ToVector(SDistanceVector) _returnvalue))) (.Z (Math|Vector|BreakVector (Class|SpiceTypes|ToVector(SDistanceVector) _returnvalue)))))))
            (:Error
              (Development|PrintString 0 _errormessage_5 true true "(R=1.000000,G=0.000000,B=0.000000,A=1.000000)"))))
        (:Error
          (Development|PrintString 0 _errormessage_4 true true "(R=1.000000,G=0.000000,B=0.000000,A=1.000000)"))))))

(fn ComputingTransformationsBetweenReferenceFrames(FK)
  ;[0 0 0 1 10] Computing Transformations Between Frames (FK)
  ; APIs:
  ; furnsh_c - loads individual kernels and collections of kernels.
  ; pxform_c - returns the 3x3 matrix rotating a position vector one frame to another.
  ; sxform_c - returns the 6x6 matrix rotating a state vector from one frame to another.
  ; pxfrm2_c - returns the 3x3 matrix rotating a position vector from one frame at a specified epoch to another frame at a different epoch.
  ; Brief Example:
  ;    The following example computes orientation of the CASSINI ISS WAC
  ;    camera relative to the Saturn body-fixed frame:
  ;
  ;       SpiceDouble   et;
  ;       SpiceDouble   mat[3][3];
  ;
  ;       /*
  ;          load kernels: LSK, PCK, CASSINI SCLK, FK and CK
  ;       */
  ;       furnsh_c ( "naif0008.tls" );
  ;       furnsh_c ( "pck00008.tpc" );
  ;       furnsh_c ( "cas00101.tsc" );
  ;       furnsh_c ( "cas_v39.tf" );
  ;       furnsh_c ( "05362_06002ra.bc" );
  ;
  ;       /*
  ;          convert UTC to ET
  ;       */
  ;       str2et_c ( "2005-DEC-28 12:00", &et );
  ;
  ;       /*
  ;          compute orientation of CASSINI relative to J2000 frame
  ;       */
  ;       pxform_c ( "IAU_SATURN", "CASSINI_ISS_WAC", et, mat );
  ; Reference documents:
  ; frames.req - reference on Frames Kernel (FK) and Frames subsystem of SPICE
  ; kernel.req - reference on loading/unloading kernels and text kernel format
  ;
  ; https://naif.jpl.nasa.gov/pub/naif/toolkit_docs/C/info/mostused.html#E
  ;[1 1 1] Example As Given
  (Utilities|FlowControl|Sequence
    (:then_0
      (bind _errormessage (Class|Spice|FurnshList (LocalVariables|GetKernels%20To%20Load))
        (:Error
          (Development|PrintString 0 _errormessage true true "(R=1.000000,G=0.000000,B=0.000000,A=1.000000)"))))
    (:then_1
      (bind (_errormessage_2 _et) (Class|Spice|Str2et "2005-DEC-28 12:00")
        (:Success
          (bind (_errormessage_3 _rotate) (Class|Spice|Pxform "IAU_SATURN" _et "CASSINI_ISS_WAC")
            (:Success
              (bind _output_get (LocalVariables|Setmat _rotate))
              (Development|PrintString 0 (Utilities|String|ToString(Text) (Utilities|Text|FormatText "Computing Transformations Between Frames (FK): Up : {0}" (Utilities|Text|ToText(String) (Class|SpiceTypes|ToVector(SDimensionless) (Class|Spice|Mxv _output_get (Class|SpiceTypes|ToSDimensionless(Vector) (Math|Vector|MakeVector 0.0 0.0 1.0)))))))))
            (:Error
              (Development|PrintString 0 _errormessage_3 true true "(R=1.000000,G=0.000000,B=0.000000,A=1.000000)"))))
        (:Error
          (Development|PrintString 0 _errormessage_2 true true "(R=1.000000,G=0.000000,B=0.000000,A=1.000000)"))))))

(fn ComputingPositionsOfSpacecraftandNaturalBodies(SPK)
  ;[0 0 0 1 10] Computing Positions of Spacecraft and Natural Bodies (SPK)
  ; APIs:
  ; furnsh_c - loads individual kernels and collections of kernels.
  ; spkezr_c - returns the state of a target body relative to an observing body.
  ; spkpos_c - returns the position of a target body relative to an observing body.
  ; spkcpo_c - returns the state of a target body relative to a constant-position observer location.
  ; spkcpt_c - returns the state of a constant-position target location relative to an observing body.
  ; spkcvo_c - returns the state of a target body relative to a constant-velocity observer location.
  ; spkcvt_c - returns the state of a constant-velocity target location relative to an observing body.
  ; spkobj_c - finds the set of ID codes for all objects in a specified SPK file.
  ; spkcov_c - finds the coverage window for a specified object in a specified SPK file.
  ; Brief Example:
  ;    The following example computes the geometric state (position and
  ;    velocity) of MGS relative to Mars in the J2000 reference frame:
  ;
  ;       SpiceDouble   et;
  ;       SpiceDouble   state[6];
  ;       SpiceDouble   lt;
  ;
  ;       /*
  ;          load kernels: LSK and MGS and DE SPKs
  ;       */
  ;       furnsh_c ( "naif0008.tls" );
  ;       furnsh_c ( "de405.bsp" );
  ;       furnsh_c ( "mgs_ext22.bsp" );
  ;
  ;       /*
  ;          convert UTC to ET
  ;       */
  ;       str2et_c ( "2006 JAN 31 01:00", &et );
  ;
  ;       /*
  ;          compute geometric state of MGS relative to Mars
  ;       */
  ;       spkezr_c ( "MGS", et, "J2000", "NONE", "MARS", state,
  ;                  &lt );
  ; Reference documents:
  ; spk.req - reference on Spacecraft and Planet Ephemeris (SPK) subsystem of SPICE
  ; frames.req - reference on Frames Kernel (FK) and Frames subsystem of SPICE
  ; kernel.req - reference on loading/unloading kernels and text kernel format
  ;
  ; https://naif.jpl.nasa.gov/pub/naif/toolkit_docs/C/info/mostused.html#F
  ;[1 1 1] Example as given
  (bind _errormessage (Class|Spice|FurnshList (LocalVariables|GetKernels%20To%20Load))
    (:Success
      (bind (_errormessage_2 _et) (Class|Spice|Str2et "2006 JAN 31 01:00")
        (:Success
          (bind (_errormessage_3 _state) (Class|Spice|Spkezr _et "MGS" "MARS" "J2000" "None")
            (:Success
              (Development|PrintString 0 (Utilities|String|ToString(Text) (Utilities|Text|FormatText "Computing Positions of Spacecraft and Natural Bodies (SPK) State Vector:  r : ({r}) km;  v : ({v}) km/s" (Utilities|Text|ToText(String) (Class|SpiceTypes|ToVector(SDistanceVector) (.r (Utilities|Struct|BreakSStateVector _state)))) (Utilities|Text|ToText(String) (Class|SpiceTypes|ToVector(SVelocityVector) (.v (Utilities|Struct|BreakSStateVector _state))))))))
            (:Error
              (Development|PrintString 0 _errormessage_3 true true "(R=1.000000,G=0.000000,B=0.000000,A=1.000000)"))))
        (:Error
          (Development|PrintString 0 _errormessage_2 true true "(R=1.000000,G=0.000000,B=0.000000,A=1.000000)"))))
    (:Error
      (Development|PrintString 0 _errormessage true true "(R=1.000000,G=0.000000,B=0.000000,A=1.000000)"))))

(fn ComputingOrientationsOfSpacecraftandInstruments(CK)
  ;[0 0 0 1 10] Computing Orientation for Spacecraft and Instruments (CK)
  ; APIs:
  ; furnsh_c - loads individual kernels and collections of kernels.
  ; pxform_c - returns the 3x3 matrix rotating a position vector one frame to another.
  ; sxform_c - returns the 6x6 matrix rotating a state vector from one frame to another.
  ; ckobj_c - finds the set of ID codes for all objects in a specified CK file.
  ; ckcov_c - finds the coverage window for a specified object in a specified CK file.
  ; ckgp_c - gets pointing for a specified CK ID at a specified SCLK time.
  ; ckgpav_c - gets pointing and angular velocity for a specified CK ID at a specified SCLK time.
  ; Brief Example:
  ;    The following example computes orientation of the CASSINI spacecraft
  ;    provided in CK files using the Frames subsystem routine pxform_c:
  ;
  ;       SpiceDouble   et;
  ;       SpiceDouble   mat[3][3];
  ;
  ;       /*
  ;          load kernels: LSK, CASSINI SCLK, FK and CK
  ;       */
  ;       furnsh_c ( "naif0008.tls" );
  ;       furnsh_c ( "cas00101.tsc" );
  ;       furnsh_c ( "cas_v39.tf" );
  ;       furnsh_c ( "05362_06002ra.bc" );
  ;
  ;       /*
  ;          convert UTC to ET
  ;       */
  ;       str2et_c ( "2005-DEC-28 12:00", &et );
  ;
  ;       /*
  ;          compute orientation of CASSINI relative to J2000 frame
  ;       */
  ;       pxform_c ( "J2000", "CASSINI_SC_COORD", et, mat );
  ; Reference documents:
  ; ck.req - reference on spacecraft orientation (CK) subsystem of SPICE
  ; frames.req - reference on Frames Kernel (FK) and Frames subsystem of SPICE
  ; kernel.req - reference on loading/unloading kernels and text kernel format
  ;
  ; https://naif.jpl.nasa.gov/pub/naif/toolkit_docs/C/info/mostused.html#G
  ;[1 1 1] Example as given
  (bind _errormessage (Class|Spice|FurnshList (LocalVariables|GetKernels%20To%20Load))
    (:Success
      (bind (_errormessage_2 _et) (Class|Spice|Str2et "2005-DEC-28 12:00")
        (:Success
          (bind (_errormessage_3 _rotate) (Class|Spice|Pxform "J2000" _et "CASSINI_SC_COORD")
            (:Success
              (Development|PrintString 0 (Utilities|String|ToString(Text) (Utilities|Text|FormatText "Computing Orientation for Spacecraft and Instruments (CK) Up Vector: {up}" (Utilities|Text|ToText(String) (Class|SpiceTypes|ToVector(SDimensionless) (Class|Spice|Mxv _rotate (Utilities|Struct|MakeSDimensionlessVector 0.0 0.0 1.0))))))))
            (:Error
              (Development|PrintString 0 _errormessage_3 true true "(R=1.000000,G=0.000000,B=0.000000,A=1.000000)"))))
        (:Error
          (Development|PrintString 0 _errormessage_2 true true "(R=1.000000,G=0.000000,B=0.000000,A=1.000000)"))))
    (:Error
      (Development|PrintString 0 _errormessage true true "(R=1.000000,G=0.000000,B=0.000000,A=1.000000)"))))

(fn RetrievingInstrumentParameters(IK)
  ;[0 0 0 1 10] Retrieving Instrument Parameters (IK)
  ; APIs:
  ; furnsh_c - loads individual kernels and collections of kernels.
  ; getfov_c - returns the field-of-view (FOV) configuration for a specified instrument.
  ; gdpool_c - returns the double precision value of a kernel variable from the kernel pool.
  ; gipool_c - returns the integer value of a kernel variable from the kernel pool.
  ; gcpool_c - returns the character value of a kernel variable from the kernel pool.
  ; Brief Example:
  ;    The following example retrieves the M01 THEMIS IR camera focal
  ;    length and FOV parameters:
  ;
  ;       SpiceBoolean  found;
  ;       SpiceChar     frame[32];
  ;       SpiceChar     shape[32];
  ;       SpiceDouble   fl;
  ;       SpiceDouble   bsight[3];
  ;       SpiceDouble   bounds[4][3];
  ;       SpiceInt      n;
  ;
  ;       /*
  ;          load THEMIS IK
  ;       */
  ;       furnsh_c ( "m01_themis_v31.ti" );
  ;
  ;       /*
  ;          retrieve M01 THEMIS IR pixel size
  ;       */
  ;       gdpool_c ( "INS-53031_FOCAL_LENGTH", 0, 1, &n, &fl,
  ;                  &found );
  ;
  ;       /*
  ;          retrieve M01 THEMIS IR FOV parameters
  ;       */
  ;       getfov_c ( -53031, 4, 32, 32, shape, frame, bsight, &n,
  ;                  bounds );
  ; Reference documents:
  ; kernel.req - reference on loading/unloading kernels and text kernel format
  ;
  ; https://naif.jpl.nasa.gov/pub/naif/toolkit_docs/C/info/mostused.html#H
  ;[1 1 1] Example as Given
  (Utilities|FlowControl|Sequence
    (:then_0
      (bind _errormessage (Class|Spice|Furnsh "Content\\Spice\\Simple\\m01_themis_v31.ti")
        (:Error
          (Development|PrintString 0 _errormessage true true "(R=1.000000,G=0.000000,B=0.000000,A=1.000000)"))))
    (:then_1
      (bind _errormessage_2 (Class|Spice|GdpoolScalar "INS-53031_FOCAL_LENGTH")
        (:Error
          (Development|PrintString 0 _errormessage_2 true true "(R=1.000000,G=0.000000,B=0.000000,A=1.000000)"))))
    (:then_2
      (bind (_errormessage_3 _shape _frame _bsight _bounds) (Class|Spice|Getfov -53031)
        (:Success
          (Utilities|FlowControl|Sequence
            (:then_0
              (Development|PrintString 0 (Utilities|String|Append "Retrieving Instrument Parameters (IK) Shape: " _shape ", Frame:" _frame)))
            (:then_1
              (Development|PrintString 0 (Utilities|String|ToString(Text) (Utilities|Text|FormatText "Retrieving Instrument Parameters (IK) Bresight : {bsight}" (Utilities|Text|ToText(String) (Class|SpiceTypes|ToVector(SDimensionless) _bsight))))))
            (:then_2
              (for (_array_element _array_index) _bounds
                (Development|PrintString 0 (Utilities|String|ToString(Text) (Utilities|Text|FormatText "Retrieving Instrument Parameters (IK) Bounds {index} : {bound}" _array_index (Utilities|Text|ToText(String) (Class|SpiceTypes|ToVector(SDimensionless) _array_element)))))))))
        (:Error
          (Development|PrintString 0 _errormessage_3 true true "(R=1.000000,G=0.000000,B=0.000000,A=1.000000)"))))))

(fn ComputingSurfaceCoordinatesUsingDigitalShape(DSK)
  (Development|PrintString 0 "Computing surface coordinates using digital shape (DSK) Not implemented, waiting on a few DSK functions" true true "(R=1.000000,G=1.000000,B=1.000000,A=1.000000)"))

(fn MappingBetweenObjectNamesandNAIFIDs
  ;[0 0 0 1 10] Mapping Between Object Names and NAIF IDs
  ; APIs:
  ; furnsh_c - loads individual kernels and collections of kernels.
  ; bodc2n_c - translates the NAIF integer code of a body into a common name for that body.
  ; bodn2c_c - translates the name of a body or object to the corresponding NAIF integer ID code.
  ; Brief Example:
  ;    The following example uses bodn2c_c to get the NAIF ID for Phobos
  ;    (built into the SPICE system) and for the M01 THEMIS IR camera
  ;    (defined in the M01 FK file):
  ;
  ;       SpiceBoolean  found;
  ;       Spiceint      phobos_id;
  ;       Spiceint      themis_ir_id;
  ;
  ;       /*
  ;          load FK defining M01 name-ID mappings
  ;       */
  ;       furnsh_c ( "m01_v28.tf" );
  ;
  ;       /*
  ;          get NAIF ID for Phobos
  ;       */
  ;       bodn2c_c ( "PHOBOS", &phobos_id, &found );
  ;
  ;       /*
  ;          get NAIF ID for THEMIS IR camera
  ;       */
  ;       bodn2c_c ( "M01_THEMIS_IR", &themis_ir_id, &found );
  ; Reference documents:
  ; naif_ids.req - reference on object names and IDs supported in SPICE
  ; kernel.req - reference on loading/unloading kernels and text kernel format
  ;
  ; https://naif.jpl.nasa.gov/pub/naif/toolkit_docs/C/info/mostused.html#I
  ;[1 1 1] Example as given
  (Utilities|FlowControl|Sequence
    (:then_0
      (bind _errormessage (Class|Spice|Furnsh "Content/Spice/Simple/m01_v28.tf")
        (:Error
          (Development|PrintString 0 _errormessage true true "(R=1.000000,G=0.000000,B=0.000000,A=1.000000)"))))
    (:then_1
      (bind _code (Class|Spice|Bodn2c "PHOBOS")
        (:Found
          (Development|PrintString 0 (Utilities|String|ToString(Text) (Utilities|Text|FormatText "Mapping Between Object Names and NAIF IDs, NAIF ID for Phobos : {id}" (Math|Conversions|ToInteger(Byte) _code)))))
        (:NotFound
          (Development|PrintString 0 "NAIF ID for Phobos not found" true true "(R=1.000000,G=0.000000,B=0.000000,A=1.000000)"))))
    (:then_2
      (bind _code_2 (Class|Spice|Bodn2c "M01_THEMIS_IR")
        (:Found
          (Development|PrintString 0 (Utilities|String|ToString(Text) (Utilities|Text|FormatText "Mapping Between Object Names and NAIF IDs, NAIF ID for M01_THEMIS_IR : {id}" (Math|Conversions|ToInteger(Byte) _code_2)))))
        (:NotFound
          (Development|PrintString 0 "NAIF ID for M01_THEMIS_IR not found" true true "(R=1.000000,G=0.000000,B=0.000000,A=1.000000)"))))))

(fn MappingBetweenSurfaceNamesandNAIFIDs
  (Development|PrintString 0 "Mapping between surface names and NAIF IDs Not implemented, waiting on a few SRF functions" true true "(R=1.000000,G=1.000000,B=1.000000,A=1.000000)"))

(fn ComputingPlanetocentric,Planetodetic,andPlanetographicCoordinates
  ;[0 0 0 1 10] Computing Planetocentric, Planetodetic, and Planetographic Coordinates
  ; APIs:
  ; reclat_c - converts from rectangular to planetocentric coordinates.
  ; latrec_c - converts from planetocentric to rectangular coordinates.
  ; srfrec_c - converts from planetocentric lat/lon of a surface point on a body to rectangular coordinates.
  ; recgeo_c - converts from rectangular to geodetic coordinates.
  ; georec_c - converts from geodetic to rectangular coordinates.
  ; recpgr_c - converts from rectangular to planetographic coordinates.
  ; pgrrec_c - converts from planetographic to rectangular coordinates.
  ; Brief Example:
  ;    The following example computes the planetocentric, planetodetic and
  ;    planetographic coordinates for a point given as a Cartesian vector
  ;    with respect to Mars in the Mars body-fixed frame (IAU_MARS):
  ;
  ;       SpiceDouble   vec[3];
  ;       SpiceDouble   radii[3];
  ;       SpiceDouble   f;
  ;       SpiceDouble   pcr,   pclon, pclat;
  ;       SpiceDouble   pdalt, pdlon, pdlat;
  ;       SpiceDouble   pgalt, pglon, pglat;
  ;       SpiceInt      n;
  ;
  ;       /*
  ;          load PCK file
  ;       */
  ;       furnsh_c( "pck00008.tpc" );
  ;
  ;       /*
  ;          retrieve Mars radii
  ;       */
  ;       bodvrd_c( "MARS", "RADII", 3, &n, radii );
  ;
  ;       /*
  ;          package 3D vector
  ;       */
  ;       vpack_c ( 3373.850, -351.034, -117.267, vec );
  ;
  ;       /*
  ;          compute planetocentric coordinates
  ;       */
  ;       reclat_c( vec, &pcr, &pclon, &pclat );
  ;
  ;       /*
  ;          compute planetodetic coordinates
  ;       */
  ;       recgeo_c( vec, radii[0], f, &pdlon, &pdlat,
  ;                 &pdalt );
  ;
  ;       /*
  ;          compute planetographic coordinates
  ;       */
  ;       recpgr_c( "MARS", vec, radii[0], f, &pglon, &pglat,
  ;                 &pgalt );
  ; Reference documents:
  ; pck.req - reference on Planetary Constants Kernel (PCK) subsystem of SPICE
  ;
  ; https://naif.jpl.nasa.gov/pub/naif/toolkit_docs/C/info/mostused.html#N
  ;[1 1 1] Example as given
  (Utilities|FlowControl|Sequence
    (:then_0
      (bind _errormessage (Class|Spice|Furnsh "Content/Spice/Simple/pck00008.tpc")
        (:Error
          (Development|PrintString 0 _errormessage true true "(R=1.000000,G=0.000000,B=0.000000,A=1.000000)"))))
    (:then_1
      (bind (_errormessage_2 _returnvalue) (Class|Spice|BodvrdDistanceVector "MARS" "RADII")
        (:Success
          (LocalVariables|Setradii (.x (Utilities|Struct|BreakSDistanceVector _returnvalue)))
          ;[1 1 1] Omitted from example.  NAIF's mistake?
          (LocalVariables|Setf (ComputingDerivedGeometry|ComputeFlattening _returnvalue)))
        (:Error
          (Development|PrintString 0 _errormessage_2 true true "(R=1.000000,G=0.000000,B=0.000000,A=1.000000)"))))
    (:then_2
      (LocalVariables|Setvec (Class|SpiceTypes|ToSDistanceVector(SDimensionlessVector) (Class|Spice|Vpack 3373.85 -351.034 -117.267))))
    (:then_3
      (LocalVariables|Setpcr (.radius (Class|Spice|Reclat (LocalVariables|Getvec))))
      (LocalVariables|Setpclonlat (.lonlat (Class|Spice|Reclat (LocalVariables|Getvec))))
      (Development|PrintString 0 (Utilities|String|ToString(Text) (Utilities|Text|FormatText "Computing Planetocentric, Planetodetic, and Planetographic Coordinates - planetocentric coordinates : lon={long} lat={lat} r={r}" (Math|Conversions|ToFloat(Integer) (Utilities|Struct|BreakSAngle (.longitude (Utilities|Struct|BreakSLonLat (LocalVariables|Getpclonlat))))) (Math|Conversions|ToFloat(Integer) (Utilities|Struct|BreakSAngle (.latitude (Utilities|Struct|BreakSLonLat (LocalVariables|Getpclonlat))))) (Math|Conversions|ToFloat(Integer) (Class|SpiceTypes|ToFloat(SDistance) (LocalVariables|Getpcr)))))))
    (:then_4
      (LocalVariables|Setpdlonlat (.lonlat (Class|Spice|Recgeo (LocalVariables|Getvec) (LocalVariables|Getradii) (LocalVariables|Getf))))
      (LocalVariables|Setpdalt (.alt (Class|Spice|Recgeo (LocalVariables|Getvec) (LocalVariables|Getradii) (LocalVariables|Getf))))
      (Development|PrintString 0 (Utilities|String|ToString(Text) (Utilities|Text|FormatText "Computing Planetocentric, Planetodetic, and Planetographic Coordinates - planetodetic coordinates : lon={long} lat={lat} alt={alt}" (Math|Conversions|ToFloat(Integer) (Utilities|Struct|BreakSAngle (.longitude (Utilities|Struct|BreakSLonLat (LocalVariables|Getpdlonlat))))) (Math|Conversions|ToFloat(Integer) (Utilities|Struct|BreakSAngle (.latitude (Utilities|Struct|BreakSLonLat (LocalVariables|Getpdlonlat))))) (Math|Conversions|ToFloat(Integer) (Class|SpiceTypes|ToFloat(SDistance) (LocalVariables|Getpdalt)))))))
    (:then_5
      (bind (_errormessage_3 _lonlat _alt) (Class|Spice|Recpgr (LocalVariables|Getvec) (LocalVariables|Getradii) "MARS" (LocalVariables|Getf))
        (:Success
          (LocalVariables|Setpglonlat _lonlat)
          (LocalVariables|Setpgalt _alt)
          (Development|PrintString 0 (Utilities|String|ToString(Text) (Utilities|Text|FormatText "Computing Planetocentric, Planetodetic, and Planetographic Coordinates - planetographic coordinates : lon={long} lat={lat} alt={alt}" (Math|Conversions|ToFloat(Integer) (Utilities|Struct|BreakSAngle (.longitude (Utilities|Struct|BreakSLonLat (LocalVariables|Getpglonlat))))) (Math|Conversions|ToFloat(Integer) (Utilities|Struct|BreakSAngle (.latitude (Utilities|Struct|BreakSLonLat (LocalVariables|Getpglonlat))))) (Math|Conversions|ToFloat(Integer) (Class|SpiceTypes|ToFloat(SDistance) (LocalVariables|Getpgalt)))))))
        (:Error
          (Development|PrintString 0 _errormessage_3 true true "(R=1.000000,G=0.000000,B=0.000000,A=1.000000)"))))))

(fn ComputingSurfaceInterceptPoint
  (Development|PrintString 0 "Computing Surface Intercept Point Not implemented, waiting on a few DSK functions" true true "(R=1.000000,G=1.000000,B=1.000000,A=1.000000)"))

(fn ComputingSub-observerandSub-solarPoints
  (Development|PrintString 0 "Computing Sub-observer and Sub-solar Points Not implemented, waiting on a few DSK functions" true true "(R=1.000000,G=1.000000,B=1.000000,A=1.000000)"))

(fn ComputingIlluminationAngles
  ;[0 0 0 1 10] Computing Illumination Angles
  ; APIs:
  ; ilumin_c - computes the illumination angles at a specified surface point of a target body, modeled as an ellipsoid or a digital shape (DSK), as seen from an observer body, illuminated by the Sun.
  ; illumg_c - computes the illumination angles at a specified surface point of a target body, modeled as an ellipsoid or a digital shape (DSK), as seen from an observer body, illuminated by a user specified body.
  ; illumf_c - computes the illumination angles at a specified surface point of a target body, modeled as an ellipsoid or a digital shape (DSK), as seen from an observer body, illuminated by a user specified body, with flags indicating whether the point is visible from the observer and whether it is illuminated.
  ; phaseq_c - computes the apparent phase angle between the centers of target, observer, and illuminator ephemeris objects.
  ; Brief Example:
  ;    The following example computes the illumination angles for a point
  ;    specified using planetocentric coordinates, observed by MGS:
  ;
  ;       SpiceDouble   r   = 3390.42;
  ;       SpiceDouble   lon =  175.30;
  ;       SpiceDouble   lat =  -14.59;
  ;       SpiceDouble   point[3];
  ;       SpiceDouble   et;
  ;       SpiceDouble   srfvec[3];
  ;       SpiceDouble   trgepc;
  ;       SpiceDouble   phase, solar, emissn;
  ;
  ;       /*
  ;          load kernels: LSK, PCK, planet/satellite SPK
  ;          and MGS spacecraft SPK
  ;       */
  ;       furnsh_c ( "naif0008.tls" );
  ;       furnsh_c ( "mars_iau2000_v0.tpc" );
  ;       furnsh_c ( "mar063.bsp" );
  ;       furnsh_c ( "mgs_ext22.bsp" );
  ;
  ;       /*
  ;          convert planetocentric r/lon/lat to Cartesian vector
  ;       */
  ;       latrec_c( r, lon * rpd_c(), lat * rpd_c(), point );
  ;
  ;       /*
  ;          convert UTC to ET
  ;       */
  ;       str2et_c ( "2006 JAN 31 01:00", &et );
  ;
  ;       /*
  ;          compute illumination angles, modeling Mars as
  ;          an ellipsoid
  ;       */
  ;       ilumin_c ( "Ellipsoid", "MARS",  et, "IAU_MARS",
  ;                  "LT+S", "MGS", point,
  ;                  &trgepc, srfvec, &phase, &solar, &emissn );
  ;
  ; https://naif.jpl.nasa.gov/pub/naif/toolkit_docs/C/info/mostused.html#L
  ;[1 1 1] Example, as given
  (Utilities|FlowControl|Sequence
    (:then_0
      (Class|Spice|FurnshList (LocalVariables|GetKernels%20To%20Load)
        (:Error
          (Development|PrintString 0 "Computing illumination angles  : mar063.bsp exceeds github max size and is not stored in git" true true "(R=1.000000,G=1.000000,B=0.000000,A=1.000000)")
          (Development|PrintString 0 "To run this example, download mar063.bsp here: https://naif.jpl.nasa.gov/pub/naif/generic_kernels/spk/satellites/a_old_versions/ and place in Content/Spice/Simple directory" true true "(R=1.000000,G=1.000000,B=0.000000,A=1.000000)")
          (return))))
    (:then_1
      (bind (_errormessage _et) (Class|Spice|Str2et "2006 JAN 31 01:00")
        (:Success
          (bind (_errormessage_2 _trgepc _srfvec _phase _incdnc _emissn) (Class|Spice|Ilumin (Class|Spice|Latrec (LocalVariables|Getr) (LocalVariables|Getlonlat)) _et "ELLIPSOID" "MARS" "IAU_MARS" "LT_S" "MGS")
            (:Success
              (bind _utcstr (Class|Spice|Et2utc _trgepc "Calendar")
                (:Success
                  (Development|PrintString 0 (Utilities|String|ToString(Text) (Utilities|Text|FormatText "Computing Illumination Angles Epoch {epoch}; srfvec {srfvec} km; phase {phase}; solar {solar}; emissn {emissn}" _utcstr (Utilities|Text|ToText(String) (Class|SpiceTypes|ToVector(SDimensionless) (Class|SpiceTypes|ToSDimensionlessVector(SDistanceVector) _srfvec))) (Math|Conversions|ToFloat(Integer) (Utilities|Struct|BreakSAngle _phase)) (Math|Conversions|ToFloat(Integer) (Utilities|Struct|BreakSAngle _incdnc)) (Math|Conversions|ToFloat(Integer) (Utilities|Struct|BreakSAngle _emissn))))))))
            (:Error
              (Development|PrintString 0 _errormessage_2 true true "(R=1.000000,G=0.000000,B=0.000000,A=1.000000)"))))
        (:Error
          (Development|PrintString 0 _errormessage true true "(R=1.000000,G=0.000000,B=0.000000,A=1.000000)"))))))

(fn ComputingLimbandTerminator
  (Development|PrintString 0 "Computing limb and terminator Not implemented, waiting on a few DSK functions" true true "(R=1.000000,G=1.000000,B=1.000000,A=1.000000)"))

(fn ComputingandPropagatingOrbitalElements
  ;[0 0 0 1 10] Computing and Propagating Orbital Elements
  ; APIs:
  ; conics_c - determines the state of an orbiting body from a set orbital elements.
  ; oscelt_c - determines the set of orbital elements corresponding to the state of a body.
  ; Brief Example:
  ;    The following example computes the set of orbital elements for the
  ;    state of the Mars Express spacecraft at a given time:
  ;
  ;       SpiceInt      n;
  ;       SpiceDouble   gm;
  ;       SpiceDouble   et;
  ;       SpiceDouble   state[6];
  ;       SpiceDouble   lt;
  ;       SpiceDouble   elts[8];
  ;
  ;       /*
  ;          load kernels: LSK, MEX trajectory SPK, and gravity PCK
  ;       */
  ;       furnsh_c ( "naif0008.tls" );
  ;       furnsh_c ( "ORMM__050901000000_00165.BSP" );
  ;       furnsh_c ( "DE403-MASSES.TPC" );
  ;
  ;       /*
  ;          retrieve GM for Mars
  ;       */
  ;       bodvrd_c ( "MARS", "GM", 1, &n, gm );
  ;
  ;       /*
  ;          convert UTC to ET
  ;       */
  ;       str2et_c ( "2005 SEP 02 04:50:45", &et );
  ;
  ;       /*
  ;          compute state of MEX at given UTC
  ;       */
  ;       spkezr_c ( "MEX", et, "MARSIAU", "NONE", "MARS",
  ;                  state, &lt );
  ;
  ;       /*
  ;          compute orbital elements
  ;       */
  ;       oscelt_c ( state, et, gm, elts );
  ;
  ; https://naif.jpl.nasa.gov/pub/naif/toolkit_docs/C/info/mostused.html#M
  ;[1 1 1] Example as given
  (Utilities|FlowControl|Sequence
    (:then_0
      (Class|Spice|FurnshList (LocalVariables|GetKernels%20To%20Load)))
    (:then_1
      (bind _returnvalue (Class|Spice|BodvrdMass "MARS" "GM")
        (:Success
          (LocalVariables|Setgm _returnvalue))))
    (:then_2
      (bind _et (Class|Spice|Str2et "2005 SEP 02 04:50:45")
        (:Success
          (LocalVariables|Setet _et))))
    (:then_3
      (bind _state (Class|Spice|Spkezr (LocalVariables|Getet) "MEX" "MARS" "MARSIAU" "None")
        (:Success
          (bind _output_get (LocalVariables|Setelts (Class|Spice|Oscelt _state (LocalVariables|Getet) (LocalVariables|Getgm))))
          (bind _utcstr (Class|Spice|Et2utc (.Epoch (Utilities|Struct|BreakSConicElements _output_get)) "Calendar")
            (:Success
              (Development|PrintString 0 (Utilities|String|ToString(Text) (Utilities|Text|FormatText "Computing and Propagating Orbital Elements rp {rp} km; ecc {ecc}; inc {inc}; lon {lon}; argpe {argpe}; epoch {epoch}; ma {ma}  " (Utilities|String|ToString(Float) (Utilities|Struct|BreakSDistance (.PerifocalDistance (Utilities|Struct|BreakSConicElements _output_get)))) (Utilities|String|ToString(Float) (.Eccentricity (Utilities|Struct|BreakSConicElements _output_get))) (Utilities|String|ToString(Float) (Utilities|Struct|BreakSAngle (.Inclination (Utilities|Struct|BreakSConicElements _output_get)))) (Utilities|String|ToString(Float) (Utilities|Struct|BreakSAngle (.LongitudeOfAscendingNode (Utilities|Struct|BreakSConicElements _output_get)))) (Utilities|String|ToString(Float) (Utilities|Struct|BreakSAngle (.ArgumentOfPeriapse (Utilities|Struct|BreakSConicElements _output_get)))) _utcstr (Utilities|String|ToString(Float) (Utilities|Struct|BreakSAngle (.MeanAnomalyAtEpoch (Utilities|Struct|BreakSConicElements _output_get))))))))))))))

(fn CheckingforinField-Of-View(FOV)Conditions)

(fn CheckingforOccultationConditions)

(fn FindingTimesOfEventsSatisfyingNumericalConstraints)

(fn FindingTimesOfEventsSatisfyingFOVConstraints)

(fn FindingTimesOfOccultations)

(fn ConvertingfromandtoRectangularCoordinates)

(fn ConvertingfromandtoSphericalCoordinates)

(fn ConvertingfromandtoCylindricalCoordinates)

(fn ConvertingfromandtoLatitudinalCoordinates)

(fn ConvertingfromandtoR,RA,DEC)

(fn ConvertingfromandtoGeodeticCoordinates)

(fn TransformingStatesfromOneCoordinateSystemtoAnother)

(fn PerformingSimpleOperationson3DVectors)

(fn PerformingSimpleOperationson3x3Matrices)

(fn Projecting,CombiningandRotating3DVectors)

(fn CreatingandConvertingTransformationMatrices)

(fn AccessingPhysicalandMathematicalConstants)

(fn ComputeFlattening
  (params (Radii :type S%20Distance%20Vector%20Structure%20%28by%20ref%29))
  (bind _returnvalue (Class|SpiceTypes|ToSDimensionlessVector(SDistanceVector) Radii))
  (bind (_x _y _z) (Utilities|Struct|BreakSDimensionlessVector _returnvalue))
  (return (/ (- _x _z) _x)))